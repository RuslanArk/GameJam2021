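; Calendar and clock Blueprint for Cloudscape Seasons that keeps game time and date, seeded at BeginPlay from system time or custom values.
; When enabled, Tick optionally recaptures the Skylight at intervals and, with auto-advance, scales delta time by day duration into a 24-hour Clockwork value.
; Clock derives time strings and a numeric TimeValue, while Calendar rolls whole-day overflow into months and years.
; Construction converts latitude and longitude to decimal degrees.
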(event EventBeginPlay
  (bind _returnvalue (Math|DateTime|Now))
  (bind _returnvalue_2 (Math|DateTime|Now))
  (if (Variables|Default|GetUseSystemDateTime)
    ;[1 1 1] System Time
    (Variables|Default|SetClockwork (+ (Math|Conversions|ToFloat(Integer) (Class|KismetMathLibrary|GetHour _returnvalue)) (/ (Math|Conversions|ToFloat(Integer) (Class|KismetMathLibrary|GetMinute _returnvalue)) 6e+01) (/ (Math|Conversions|ToFloat(Integer) (Class|KismetMathLibrary|GetSecond _returnvalue)) 3.6e+03)))
    (Variables|Default|SetDay (Class|KismetMathLibrary|GetDay _returnvalue_2))
    (Variables|Default|SetMonth (Class|KismetMathLibrary|GetMonth _returnvalue_2))
    (Variables|Default|SetYear (Class|KismetMathLibrary|GetYear _returnvalue_2))
    (else
      ;[1 1 1] Custom Time
      (Variables|Default|SetClockwork (+ (Math|Conversions|ToFloat(Integer) (Variables|Default|GetHour)) (/ (Math|Conversions|ToFloat(Integer) (Variables|Default|GetMinutes)) 6e+01) (/ (Math|Conversions|ToFloat(Integer) (Variables|Default|GetSeconds)) 3.6e+03)))))
  ;[1 1 1] Setting Game Date for Display
  (Variables|Default|SetGameDate (Utilities|Array|MakeArray (Variables|Default|GetDay) (Variables|Default|GetMonth) (Variables|Default|GetYear))))

(event EventTick
  (params (DeltaSeconds :type Float%20%28single-precision%29))
  (bind _skylight (Variables|Default|GetSkylight))
  ;[1 1 1] Driving Clock
  (if (Variables|Default|GetEnabled)
    (if (Variables|Default|GetUpdate%20Skylight%20regularly)
      (Utilities|IsValid _skylight
        (:Is%20Valid
          (bind _output_get (Variables|Default|SetLastUpdate (+ DeltaSeconds (Variables|Default|GetLastUpdate))))
          (if (>= _output_get (Variables|Default|GetSkylight%20update%20interval))
            (Variables|Default|SetLastUpdate 0.0)
            (Class|SkyLightComponent|RecaptureSky (Variables|/Script/Engine.SkyLight|GetLightComponent _skylight) :!label _label)
            (else
              (Utilities|FlowControl|Sequence
                (:then_0
                  (Utilities|FlowControl|DoOnce false
                    (:Completed
                      (goto _label))))
                (:then_1
                  _)))))
        (:Is%20Not%20Valid
          _)))
    (if (Variables|Default|GetAutoAdvanceTime)
      (Variables|Default|SetClockwork (.Remainder (Math|Float|Division(WholeandRemainder) (+ (* (/ (/ DeltaSeconds (Variables|Default|GetTimeUnit)) (Variables|Default|GetSunDayDuration)) 24.0) (Variables|Default|GetClockwork)) 24.0)))
      (Variables|Default|SetDayTick (.ReturnValue (Math|Float|Division(WholeandRemainder) (+ (* (/ (/ DeltaSeconds (Variables|Default|GetTimeUnit)) (Variables|Default|GetSunDayDuration)) 24.0) (Variables|Default|GetClockwork)) 24.0)))
      ;[1 1 1] Updating Clock and Calendar
      (CallFunction|Clock)
      (CallFunction|Calendar))))

(fn ConstructionScript
  (Variables|Default|SetLatitude (CallFunction|DMStoDecimal (Variables|Default|GetLatitude%20Degrees) (Variables|Default|GetLatitude%20Minutes) (Variables|Default|GetLatitude%20Seconds)))
  (Variables|Default|SetLongitude (CallFunction|DMStoDecimal (Variables|Default|GetLongitude%20Degrees) (Variables|Default|GetLongitude%20Minutes) (Variables|Default|GetLongitude%20Seconds))))

(fn Clock
  (bind _clockwork (Variables|Default|GetClockwork))
  (bind _returnvalue (* _clockwork 3.6e+03))
  (bind (_remainder _returnvalue_2) (Math|Float|Division(WholeandRemainder) _returnvalue 6e+01))
  (bind _returnvalue_3 (Math|Conversions|ToFloat(Integer) _returnvalue_2))
  (bind (_remainder_2 _returnvalue_4) (Math|Float|Division(WholeandRemainder) _returnvalue_3 6e+01))
  (bind _output_get (Variables|Default|SetSeconds (Math|Float|Floor _remainder)))
  (bind _output_get_2 (Variables|Default|SetMinutes (Math|Float|Floor _remainder_2)))
  (bind _output_get_3 (Variables|Default|SetHour (Math|Float|Floor (.Remainder (Math|Float|Division(WholeandRemainder) (Math|Conversions|ToFloat(Integer) _returnvalue_4) 24.0)))))
  (bind _output_get_4 (Variables|Default|SetGameTime (Utilities|Array|MakeArray _output_get _output_get_2 _output_get_3)))
  (if (== (Utilities|String|Len (Utilities|String|ToString(Integer) (Utilities|Array|Get(acopy) _output_get_4 2))) 1)
    (Variables|Default|SettmpValHour (Utilities|String|Append "0" (Utilities|String|ToString(Integer) (Utilities|Array|Get(acopy) _output_get_4 2)) ":"))
    (else
      (Variables|Default|SettmpValHour (Utilities|String|Append (Utilities|String|ToString(Integer) (Utilities|Array|Get(acopy) _output_get_4 2)) ":"))))
  (if (== (Utilities|String|Len (Utilities|String|ToString(Integer) (Utilities|Array|Get(acopy) _output_get_4 1))) 1)
    (Variables|Default|SettmpValMin (Utilities|String|Append "0" (Utilities|String|ToString(Integer) (Utilities|Array|Get(acopy) _output_get_4 1)) ":"))
    (else
      (Variables|Default|SettmpValMin (Utilities|String|Append (Utilities|String|ToString(Integer) (Utilities|Array|Get(acopy) _output_get_4 1)) ":"))))
  (if (== (Utilities|String|Len (Utilities|String|ToString(Integer) (Utilities|Array|Get(acopy) _output_get_4))) 1)
    (Variables|Default|SettmpValSec (Utilities|String|Append "0" (Utilities|String|ToString(Integer) (Utilities|Array|Get(acopy) _output_get_4))))
    (else
      (Variables|Default|SettmpValSec (Utilities|String|ToString(Integer) (Utilities|Array|Get(acopy) _output_get_4)))))
  (Variables|Default|SetGameTimeString (Utilities|String|Append (Variables|Default|GettmpValHour) (Variables|Default|GettmpValMin) (Variables|Default|GettmpValSec)))
  (Variables|Default|SetTimeValue (|(((((({C42A1833-48DF-1344-D4B1-A292BDCB439B}*2147483647)+({ADE70DAE-40B3-9066-B916-BBB7755CFF37}*100000000))+({CE4B98CB-47D9-2747-D6DB-D1AE76E77F70}*1000000))+({12AAFABD-4E9F-D6B7-540A-09B3FCE775C2}*10000))+({12EF99B3-40BB-1667-D3ED-F99F3C970BC5}*100))+{F7632185-49A8-2ECF-4B56-87B8B82910B3}))))

(fn Calendar
  (Variables|Default|SetDay (+ (Variables|Default|GetDay) (Variables|Default|GetDayTick)))
  (if (> (Variables|Default|GetDay) (Class|KismetMathLibrary|DaysinMonth (Utilities|Array|Get(acopy) (Variables|Default|GetGameDate) 2) (Utilities|Array|Get(acopy) (Variables|Default|GetGameDate) 1)))
    (Variables|Default|SetDay 1)
    (Variables|Default|SetMonth (+ (Variables|Default|GetMonth) 1)))
  (if (> (Variables|Default|GetMonth) 12)
    (Variables|Default|SetMonth 1)
    (Variables|Default|SetYear (+ (Variables|Default|GetYear) 1)))
  (Variables|Default|SetGameDate (Utilities|Array|MakeArray (Variables|Default|GetDay) (Variables|Default|GetMonth) (Variables|Default|GetYear)))
  (Variables|Default|SetGameDateString (Utilities|String|BuildString(Integer) (Utilities|String|BuildString(Integer) (Utilities|String|ToString(Integer) (Utilities|Array|Get(acopy) (Variables|Default|GetGameDate))) "-" (Utilities|Array|Get(acopy) (Variables|Default|GetGameDate) 1)) "-" (Utilities|Array|Get(acopy) (Variables|Default|GetGameDate) 2))))

(fn DMStoDecimal
  (params (Degrees :type Float%20%28single-precision%29) (Minutes :type Float%20%28single-precision%29) (Secons :type Float%20%28single-precision%29))
  (return (+ Degrees (/ Minutes 6e+01) (/ Secons 3.6e+03))))