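; Moon actor for Cloudscape Seasons that rotates a movable Moonlight and calculates the current moon phase from a Calendar's date, time and location.
; Updates run on construction, at BeginPlay and, when enabled, at a set Tick interval.
; The Calendar's TimeEvolution selects an astronomical latitude/longitude trajectory, a simple time-mapped circular path, or a stored rotation.
; Julian-day math expressions derive lunar altitude, azimuth and phase.
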(event Custom|UpdateMoon
  (bind _moonlight (Variables|Default|GetMoonlight))
  (Utilities|IsValid _moonlight
    (:Is%20Valid
      (if (Utilities|Enum|Equal(Enum) (Variables|/Script/Engine.SceneComponent|GetMobility (Variables|/Script/Engine.Light|GetLightComponent _moonlight)) "Movable")
        (CallFunction|UpdateDateTime)
        (CallFunction|UpdateTrajectory)
        (CallFunction|UpdateMoonPhase)))))

(event EventBeginPlay
  (CallFunction|UpdateMoon))

(event EventTick
  (params (DeltaSeconds :type Float%20%28single-precision%29))
  (if (Variables|Default|GetEnabled)
    (bind _output_get (Variables|Default|SetLastUpdate (+ DeltaSeconds (Variables|Default|GetLastUpdate))))
    (if (>= _output_get (Variables|Default|GetTrajectoryUpdateInterval))
      (Variables|Default|SetLastUpdate 0.0)
      (CallFunction|UpdateMoon))))

(fn ConstructionScript
  (if (Variables|Default|GetRefresh)
    _
    (else
      _))
  (Variables|Default|SetRefresh false)
  (CallFunction|UpdateMoon))

(fn UpdateTrajectory
  (bind _calendar (Variables|Default|GetCalendar))
  (bind _time_evolution (Variables|/Game/CloudscapeSeasons/Blueprints/BP_CalendarSeasons.BP_CalendarSeasons_C|GetTime%20Evolution _calendar))
  (Utilities|IsValid (Variables|Default|GetMoonlight)
    (:Is%20Valid
      (Utilities|IsValid _calendar
        (:Is%20Valid
          (if (Utilities|Enum|Equal(Enum) _time_evolution "NewEnumerator0")
            ;[1 1 1] Longitude/Latitude Based Trajectory
            (Transformation|SetWorldRotation (Variables|/Script/Engine.Light|GetLightComponent (Variables|Default|GetMoonlight)) (CallFunction|CalculateTrajectory (Variables|Default|GetLatitude) (Variables|Default|GetLongitude) (Variables|Default|GetHour) (Variables|Default|GetMinute) (Variables|Default|GetSecond) (Variables|Default|GetYear) (Variables|Default|GetMonth) (Variables|Default|GetDay) (Variables|Default|GetDST)) false false)
            (elif (Utilities|Enum|Equal(Enum) _time_evolution "NewEnumerator1")
              ;[1 1 1] Circular Based Trajectory
              (Transformation|SetWorldRotation (Variables|/Script/Engine.Light|GetLightComponent (Variables|Default|GetMoonlight)) (CallFunction|CalculateTrajectoryCircular (Variables|Default|GetHour) (Variables|Default|GetMinute) (Variables|Default|GetSecond)) false false)
              (elif (Utilities|Enum|Equal(Enum) _time_evolution "NewEnumerator2")
                (Transformation|SetWorldRotation (Variables|/Script/Engine.Light|GetLightComponent (Variables|Default|GetMoonlight)) (Variables|Default|GetRotator) false false)))))))))

(fn UpdateDateTime
  (bind _calendar (Variables|Default|GetCalendar))
  (Utilities|IsValid _calendar
    (:Is%20Valid
      (Variables|Default|SetDST (Variables|/Game/CloudscapeSeasons/Blueprints/BP_CalendarSeasons.BP_CalendarSeasons_C|GetDST _calendar))
      (Variables|Default|SetLatitude%20Degrees (Variables|/Game/CloudscapeSeasons/Blueprints/BP_CalendarSeasons.BP_CalendarSeasons_C|GetLatitude%20Degrees _calendar))
      (Variables|Default|SetLatitude%20Minutes (Variables|/Game/CloudscapeSeasons/Blueprints/BP_CalendarSeasons.BP_CalendarSeasons_C|GetLatitude%20Minutes _calendar))
      (Variables|Default|SetLatitude%20Seconds (Variables|/Game/CloudscapeSeasons/Blueprints/BP_CalendarSeasons.BP_CalendarSeasons_C|GetLatitude%20Seconds _calendar))
      (Variables|Default|SetLongitude%20Degrees (Variables|/Game/CloudscapeSeasons/Blueprints/BP_CalendarSeasons.BP_CalendarSeasons_C|GetLongitude%20Degrees _calendar))
      (Variables|Default|SetLongitude%20Minutes (Variables|/Game/CloudscapeSeasons/Blueprints/BP_CalendarSeasons.BP_CalendarSeasons_C|GetLongitude%20Minutes _calendar))
      (Variables|Default|SetLongitude%20Seconds (Variables|/Game/CloudscapeSeasons/Blueprints/BP_CalendarSeasons.BP_CalendarSeasons_C|GetLongitude%20Seconds _calendar))
      (Variables|Default|SetLatitude (Variables|/Game/CloudscapeSeasons/Blueprints/BP_CalendarSeasons.BP_CalendarSeasons_C|GetLatitude _calendar))
      (Variables|Default|SetLongitude (Variables|/Game/CloudscapeSeasons/Blueprints/BP_CalendarSeasons.BP_CalendarSeasons_C|GetLongitude _calendar))
      (Variables|Default|SetYear (Variables|/Game/CloudscapeSeasons/Blueprints/BP_CalendarSeasons.BP_CalendarSeasons_C|GetYear _calendar))
      (Variables|Default|SetMonth (Variables|/Game/CloudscapeSeasons/Blueprints/BP_CalendarSeasons.BP_CalendarSeasons_C|GetMonth _calendar))
      (Variables|Default|SetDay (Variables|/Game/CloudscapeSeasons/Blueprints/BP_CalendarSeasons.BP_CalendarSeasons_C|GetDay _calendar))
      (Variables|Default|SetHour (Variables|/Game/CloudscapeSeasons/Blueprints/BP_CalendarSeasons.BP_CalendarSeasons_C|GetHour _calendar))
      (Variables|Default|SetMinute (Variables|/Game/CloudscapeSeasons/Blueprints/BP_CalendarSeasons.BP_CalendarSeasons_C|GetMinutes _calendar))
      (Variables|Default|SetSecond (Variables|/Game/CloudscapeSeasons/Blueprints/BP_CalendarSeasons.BP_CalendarSeasons_C|GetSeconds _calendar)))))

(fn UpdateMoonPhase
  (Variables|Default|SetCurrentMoonPhase (CallFunction|CalculateMoonPhase (Variables|Default|GetYear) (Variables|Default|GetMonth) (Variables|Default|GetDay))))

(fn CalculateTrajectory
  (params (Latitude :type Float%20%28single-precision%29) (Longitude :type Float%20%28single-precision%29) (Hour :type Integer) (Minute :type Integer) (Second :type Integer) (Year :type Integer) (Month :type Integer) (Day :type Integer) (DST :type Boolean))
  (bind _returnvalue (|({749C384A-4B19-4268-91F9-7BAC62820DCF}+{2243651C-44B4-89E5-6807-5286780050CF})))
  (Utilities|FlowControl|Sequence
    (:then_0
      ;[1 1 1] Step 1
      (Variables|Default|Setdate (Math|DateTime|MakeDateTime Year Month Day Hour Minute Second))
      (LocalVariables|SetbDST DST))
    (:then_1
      ;[1 1 1] Step 2
      (Variables|Default|SetDayOfYear (Math|Conversions|ToFloat(Integer) (- (Class|KismetMathLibrary|GetDayOfYear (Variables|Default|Getdate)) 1))))
    (:then_2
      ;[1 1 1] Step 3
      (if (LocalVariables|GetbDST)
        (Variables|Default|SetOffsetUTC 1.0)
        (Variables|Default|SetOffsetDST 1.0)
        (else
          (Variables|Default|SetOffsetUTC 0.0)
          (Variables|Default|SetOffsetDST 0.0)))
      (Variables|Default|Setutc 0.0))
    (:then_3
      ;[1 1 1] Step 4
      (Variables|Default|SetLSTM (|(15.000000*{80408A01-4D04-3EBC-6397-5392F39A1AFC})))
      (if (LocalVariables|GetbDST)
        (Math|Float|DecrementFloat (Variables|Default|GetLSTM))))
    (:then_4
      ;[1 1 1] Step 5
      (Variables|Default|SetLct (Math|Timespan|GetTotalHours (TimeOfDay|GetTimeOfDay (Variables|Default|Getdate) :!class /Script/Engine.KismetMathLibrary))))
    (:then_5
      ;[1 1 1] Step 6
      (Variables|Default|SetSpanUTC (+ (Variables|Default|GetOffsetUTC) (Variables|Default|GetOffsetDST))))
    (:then_6
      ;[1 1 1] Step 7
      (Variables|Default|Setelapsed (- (CallFunction|GetJulianDay (Variables|Default|Getdate)) 2451545.0)))
    (:then_7
      ;[1 1 1] Step 8
      (if (> (|({749C384A-4B19-4268-91F9-7BAC62820DCF}+{2243651C-44B4-89E5-6807-5286780050CF})) 24.0)
        (Variables|Default|Setutc (- _returnvalue 24.0))
        (Math|Float|IncrementFloat (Variables|Default|Getelapsed))
        (else
          (Variables|Default|Setutc _returnvalue))))
    (:then_8
      ;[1 1 1] Step 9
      (Variables|Default|Setelapsed (|({AC1D84F6-4738-D572-15D1-E489137A3866}+({E29A5AA8-4445-E2B9-8655-5BB68CFD48F9}/24.000000)))))
    (:then_9
      ;[1 1 1] Step 10
      (Variables|Default|SetPartL (|((218.315994+(13.176396*{AC1D84F6-4738-D572-15D1-E489137A3866}))%360.000000))))
    (:then_10
      ;[1 1 1] Step 11
      (Variables|Default|SetPartM (|((134.962997+(13.064993*{AC1D84F6-4738-D572-15D1-E489137A3866}))%360.000000))))
    (:then_11
      ;[1 1 1] Step 12
      (Variables|Default|SetPartF (|((93.272003+(13.229350*{AC1D84F6-4738-D572-15D1-E489137A3866}))%360.000000))))
    (:then_12
      ;[1 1 1] Step 13
      (Variables|Default|SetecLong (|({47D429A8-4CDD-621C-1E37-C6BE06142C86}+(6.289000*(SINd({502A735F-4B51-49AE-C922-B38DD6204D3D})))))))
    (:then_13
      ;[1 1 1] Step 14
      (Variables|Default|SetecLat (|(5.128000*(SINd({11F2457A-4F33-CA83-84DB-4E8DBEDC3B8A}))))))
    (:then_14
      ;[1 1 1] Step 15
      (Variables|Default|SetecDist (|(385001.000000-(20905.000000*(COSd({502A735F-4B51-49AE-C922-B38DD6204D3D})))))))
    (:then_15
      ;[1 1 1] Step 16
      (Variables|Default|SetlunarDec (|(ASINd((((SINd({7D9017EF-459F-63D3-F786-989DAAB37A91}))*(COSd(23.439699)))+(((COSd({7D9017EF-459F-63D3-F786-989DAAB37A91}))*(SINd(23.439699)))*(SINd({3E268B65-4006-4870-176B-B5B027AEC6B3})))))))))
    (:then_16
      ;[1 1 1] Step 17
      (Variables|Default|SetlunarRA (Class|KismetMathLibrary|DegAtan2 (|(((SINd({3E268B65-4006-4870-176B-B5B027AEC6B3}))*(COSd(23.439699)))-((TANd({7D9017EF-459F-63D3-F786-989DAAB37A91}))*(SINd(23.439699))))) (|(COSd({3E268B65-4006-4870-176B-B5B027AEC6B3}))))))
    (:then_17
      ;[1 1 1] Step 18
      (Variables|Default|SetlunarST (|((((357.009003+102.936996)+(15.000000*{E29A5AA8-4445-E2B9-8655-5BB68CFD48F9}))-{47AE8D12-4C63-8F78-A873-14B28088BC95})%360.000000))))
    (:then_18
      ;[1 1 1] Step 19
      (Variables|Default|SetlunarHRA (|({671DD40F-44CD-70B5-993B-6199C8E82A4D}-{D87C9964-4A96-1AB0-1C15-1D8FEC0D633D}))))
    (:then_19
      ;[1 1 1] Step 20
      (Variables|Default|SetlunarAA (|(ASINd((((SINd({99211AF0-42B7-8C26-31A2-64A949AB99E5}))*(SINd({BE42855C-4196-81E2-366B-91943A7036D4})))+(((COSd({99211AF0-42B7-8C26-31A2-64A949AB99E5}))*(COSd({BE42855C-4196-81E2-366B-91943A7036D4})))*(COSd({D7BA9CD9-421F-34E9-7C77-E1B993EB2921})))))))))
    (:then_20
      ;[1 1 1] Step 21
      (Variables|Default|SetlunarAz (Class|KismetMathLibrary|DegAtan2 (|(SINd({D7BA9CD9-421F-34E9-7C77-E1B993EB2921}))) (|(((COSd({D7BA9CD9-421F-34E9-7C77-E1B993EB2921}))*(SINd({99211AF0-42B7-8C26-31A2-64A949AB99E5})))-((TANd({BE42855C-4196-81E2-366B-91943A7036D4}))*(COSd({99211AF0-42B7-8C26-31A2-64A949AB99E5}))))))))
    (:then_21
      ;[1 1 1] Last Step
      (bind _output_get (Variables|Default|Setresult (Math|Rotator|MakeRotator 0.0 (- (Variables|Default|GetlunarAA) 1.8e+02) (Variables|Default|GetlunarAz))))
      (return _output_get))))

(fn CalculateMoonPhase
  (params (Year :type Integer) (Month :type Integer) (Day :type Integer))
  (Utilities|FlowControl|Sequence
    (:then_0
      ;[1 1 1] Step 1
      (Variables|Default|Setdate (Math|DateTime|MakeDateTime Year Month Day)))
    (:then_1
      ;[1 1 1] Step 2
      (Variables|Default|Setene (Math|Conversions|ToFloat(Integer) (|(floor((12.370000*(({DF75FEB1-4274-EAB4-8A21-AE941E20DC88}-1900.000000)+(((1.000000*{106EDEC8-4D67-4615-E506-3193438BF455})-0.500000)/12.000000)))))))))
    (:then_2
      ;[1 1 1] Step 3
      (Variables|Default|SetRAD (|(PI/180.000000) (Math|Trig|GetPI))))
    (:then_3
      ;[1 1 1] Step 4
      (bind _output_get (Variables|Default|SetT (|({6207F1DC-4260-71ED-8085-03859D7414C6}/1236.849976))))
      (Variables|Default|SetT2 (* _output_get (Variables|Default|GetT))))
    (:then_4
      ;[1 1 1] Step 5
      (Variables|Default|SetAs (|(359.224213+(29.105356*{6207F1DC-4260-71ED-8085-03859D7414C6})))))
    (:then_5
      ;[1 1 1] Step 6
      (Variables|Default|SetAm (|((306.025299+(385.816925*{6207F1DC-4260-71ED-8085-03859D7414C6}))+(0.010730*{E773E957-4F09-7311-F6BD-A7AEE7F0A6ED})))))
    (:then_6
      ;[1 1 1] Step 7
      (bind _output_get_2 (Variables|Default|SetXtra (|((0.759330+(1.530589*{6207F1DC-4260-71ED-8085-03859D7414C6}))+(((0.117800-0.000015)*{81C74306-4197-AF54-2164-D58A835FE831})*{E773E957-4F09-7311-F6BD-A7AEE7F0A6ED})))))
      (Variables|Default|SetXtra (+ _output_get_2 (|(((0.173400-(0.039300*{81C74306-4197-AF54-2164-D58A835FE831}))*(SINd(({2D663D84-4058-A48A-DAA4-FCB7F3F8BCB2}*{A65574A9-4C2C-552D-0403-38AE4D01C1AA}))))-(0.406800*(SINd(({2D663D84-4058-A48A-DAA4-FCB7F3F8BCB2}*{87E16492-4A19-073B-84C7-AFB9151D509C})))))))))
    (:then_7
      ;[1 1 1] Step 8
      (if (> (Variables|Default|GetXtra) 0.0)
        (Variables|Default|Seti (Math|Conversions|ToFloat(Integer) (|(floor({89046354-438F-B598-12DC-91A4F3135F83})))))
        (else
          (Variables|Default|Seti (Math|Conversions|ToFloat(Integer) (|(FCeil(({89046354-438F-B598-12DC-91A4F3135F83}-1.000000)))))))))
    (:then_8
      ;[1 1 1] Step 9
      (Variables|Default|SetJ1 (CallFunction|GetJulianDay (Variables|Default|Getdate))))
    (:then_9
      ;[1 1 1] Step 10
      (Variables|Default|SetJd (|((2415020.000000+(28.000000*{6207F1DC-4260-71ED-8085-03859D7414C6}))+{68A64F14-4AC4-17A2-7C59-FBBD0F1F9A84}))))
    (:then_10
      ;[1 1 1] Last Step
      (return (|((({1263E215-4DAE-3367-4A76-C598F522FDCE}-{203E4757-4390-0554-81C9-87882B42F501})+30.000000)%30.000000))))))

(fn GetJulianDay
  (params (Date :type Date%20Time%20Structure))
  (bind (_year _month _day) (Math|DateTime|BreakDateTime Date))
  (Variables|Default|SetY (Math|Conversions|ToFloat(Integer) _year))
  (Variables|Default|SetM (Math|Conversions|ToFloat(Integer) _month))
  (Variables|Default|SetD (Math|Conversions|ToFloat(Integer) _day))
  (return (|(((({C1E9ECD1-4969-F1FE-A9EB-059E96B215B2}-32075)+((1461*(({755426A0-4106-BD17-FD0A-B69749694454}+4800)+(({691C0A06-4CA4-3224-ECF7-8FAE30DAA1F0}-14)/12)))/4))+((367*(({691C0A06-4CA4-3224-ECF7-8FAE30DAA1F0}-2)-((({691C0A06-4CA4-3224-ECF7-8FAE30DAA1F0}-14)/12)*12)))/12))-((3*((({755426A0-4106-BD17-FD0A-B69749694454}+4900)+(({691C0A06-4CA4-3224-ECF7-8FAE30DAA1F0}-14)/12))/100))/4)))))

(fn GetLongTime
  (params (Hour :type Integer) (Minute :type Integer) (Second :type Integer))
  (return (+ (Math|Conversions|ToFloat(Integer) Hour) (/ (Math|Conversions|ToFloat(Integer) Minute) 6e+01) (/ (Math|Conversions|ToFloat(Integer) Second) 3.6e+03))))

(fn CalculateTrajectoryCircular
  (params (Hour :type Integer) (Minute :type Integer) (Second :type Integer))
  (bind _longtime (CallFunction|GetLongTime Hour Minute Second))
  (bind _returnvalue (Math|Float|MapRangeClamped _longtime 0.0 11.99 -9e+01 9e+01))
  (bind _returnvalue_2 (Math|Float|MapRangeClamped _longtime 12.0 23.99 9e+01 -9e+01))
  (if (>= _longtime 12.0)
    (return (Math|Rotator|MakeRotator 0.0 _returnvalue_2 (+ _returnvalue_2 (Math|Float|MapRangeClamped _longtime 12.0 23.99 6e+01 1e+02))))
    (else
      (return (Math|Rotator|MakeRotator 0.0 _returnvalue (- _returnvalue (Math|Float|MapRangeClamped _longtime 0.0 11.99 1e+02 6e+01)))))))