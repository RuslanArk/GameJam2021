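; Cloudscape Seasons sky actor that drives a sky sphere dynamic material from assigned sun and moon directional lights.
; The construction script applies sky, cloud, star and moon parameters, optionally taking colors from curves keyed on sun height.
; Tick refreshes sun and moon at component-set intervals, can drive fog density by curve, and fades and recaptures the skylight across day/night while toggling light visibility.
; Moon texture and brightness come from a moon-phase data table.
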(event EventTick
  (params (DeltaSeconds :type Float%20%28single-precision%29))
  (bind _volumetric_fog (Variables|Sky|GetVolumetric%20Fog))
  (bind _volumetric_fog_curve (Variables|Sky|GetVolumetric%20Fog%20Curve))
  (bind _sun_light_actor (Variables|Sun|GetSun%20light%20actor))
  (bind _moon_light_actor (Variables|Moon|GetMoon%20light%20actor))
  (bind _moon_light_actor_2 (Variables|Moon|GetMoon%20light%20actor))
  (bind _sun_light_actor_2 (Variables|Sun|GetSun%20light%20actor))
  (bind _cloudscape_component (Variables|Clouds|GetCloudscape%20Component))
  (if (Variables|Default|GetEnabled)
    (Utilities|IsValid _cloudscape_component
      (:Is%20Valid
        (Utilities|FlowControl|Sequence
          (:then_0
            ;[1 1 1] Update Sun
            (bind _output_get (Variables|Default|SetLastSunUpdate (+ DeltaSeconds (Variables|Default|GetLastSunUpdate))))
            (if (>= _output_get (Variables|/Game/CloudscapeSeasons/Blueprints/BP_CloudscapeSeasons.BP_CloudscapeSeasons_C|GetSunlight%20Update%20Interval _cloudscape_component))
              (Variables|Default|SetLastSunUpdate 0.0)
              (CallFunction|UpdateSunDirection)
              ;[1 1 1] handles Volumetric Fog drive by curve
              (if (Variables|Sky|GetEnabled%20Fog%20Control%20with%20Curve) :!label _label
                (Utilities|IsValid _volumetric_fog
                  (:Is%20Valid
                    (Utilities|IsValid _volumetric_fog_curve
                      (:Is%20Valid
                        (Class|ExponentialHeightFogComponent|SetFogDensity (Variables|/Script/Engine.ExponentialHeightFog|GetComponent _volumetric_fog) (Math|Curves|GetFloatValue _volumetric_fog_curve (Variables|Overridesettings|GetSun%20height))))))))))
          (:then_1
            ;[1 1 1] Update Moon
            (bind _output_get_2 (Variables|Default|SetLastMoonUpdate (+ DeltaSeconds (Variables|Default|GetLastMoonUpdate))))
            (if (>= _output_get_2 (Variables|/Game/CloudscapeSeasons/Blueprints/BP_CloudscapeSeasons.BP_CloudscapeSeasons_C|GetMoonlight%20Update%20Interval _cloudscape_component))
              (Variables|Default|SetLastMoonUpdate 0.0)
              (CallFunction|UpdateMoonDirection)
              (goto _label)))
          (:then_2
            ;[1 1 1] Update Skly Light
            (if (Variables|DayandNight|GetUpdateDayNightTransitions)
              (Utilities|IsValid (Variables|Sky|GetSky%20Light)
                (:Is%20Valid
                  (if (< (Variables|Overridesettings|GetSun%20height) 0.0)
                    ;;[1 1 1] NightTime control
                    (Utilities|FlowControl|Sequence
                      (:then_0
                        (Variables|Default|SetNight%20Now true)
                        (Variables|Default|SetDay%20Now false))
                      (:then_1
                        (if (Variables|Sun|GetSunlight%20vanishes?)
                          (Utilities|IsValid _sun_light_actor
                            (:Is%20Valid
                              (Rendering|SetVisibility (Variables|/Script/Engine.Light|GetLightComponent _sun_light_actor) false false)))))
                      (:then_2
                        (Utilities|IsValid _moon_light_actor
                          (:Is%20Valid
                            (Rendering|SetVisibility (Variables|/Script/Engine.Light|GetLightComponent _moon_light_actor) (not (Utilities|Enum|Equal(Enum) (Variables|Moon|GetMoonPhase) "NewEnumerator0")) false))))
                      (:then_3
                        (Utilities|FlowControl|DoOnce true :!label _label_2
                          (:Completed
                            (Utilities|FlowControl|Sequence
                              (:then_0
                                (bind _intensity (Timeline|SkyLightAtNight SetNewTime)
                                  (:Update
                                    (Rendering|Components|Light|SetIntensity (Variables|/Script/Engine.SkyLight|GetLightComponent (Variables|Sky|GetSky%20Light)) (Math|Float|Lerp (Variables|DayandNight|GetLightIntensityAtNight) (Variables|DayandNight|GetLightIntensityAtDay) _intensity))
                                    (Utilities|FlowControl|DoOnce false :!label _label_3
                                      (:Completed
                                        _)))
                                  (:Finished
                                    (Utilities|FlowControl|Sequence
                                      (:then_0
                                        (goto _label_3 Reset))
                                      (:then_1
                                        _))))
                                ;;[1 1 1] Update the scene captures
                                (Class|SkyLightComponent|RecaptureSky (Variables|/Script/Engine.SkyLight|GetLightComponent (Variables|Sky|GetSky%20Light)) :!label _label_4))
                              (:then_1
                                (Timeline|SkyLightAtNight PlayFromStart))))))
                      (:then_4
                        (goto _label_5 Reset)))
                    (else
                      ;;[1 1 1] DayTime control
                      (Utilities|FlowControl|Sequence
                        (:then_0
                          (Variables|Default|SetNight%20Now false)
                          (Variables|Default|SetDay%20Now true))
                        (:then_1
                          (if (Variables|Moon|GetMoonlight%20vanishes?)
                            (Utilities|IsValid _moon_light_actor_2
                              (:Is%20Valid
                                (Rendering|SetVisibility (Variables|/Script/Engine.Light|GetLightComponent _moon_light_actor_2) false false)))))
                        (:then_2
                          (Utilities|IsValid _sun_light_actor_2
                            (:Is%20Valid
                              (Rendering|SetVisibility (Variables|/Script/Engine.Light|GetLightComponent _sun_light_actor_2) true false))))
                        (:then_3
                          (Utilities|FlowControl|DoOnce true :!label _label_5
                            (:Completed
                              (Utilities|FlowControl|Sequence
                                (:then_0
                                  (bind _intensity_2 (Timeline|SkyLightAtDay SetNewTime)
                                    (:Update
                                      (Rendering|Components|Light|SetIntensity (Variables|/Script/Engine.SkyLight|GetLightComponent (Variables|Sky|GetSky%20Light)) (Math|Float|Lerp (Variables|DayandNight|GetLightIntensityAtNight) (Variables|DayandNight|GetLightIntensityAtDay) _intensity_2))
                                      (Utilities|FlowControl|DoOnce false :!label _label_6
                                        (:Completed
                                          (goto _label_4))))
                                    (:Finished
                                      (Utilities|FlowControl|Sequence
                                        (:then_0
                                          (goto _label_6 Reset))
                                        (:then_1
                                          (goto _label_4))))))
                                (:then_1
                                  (Timeline|SkyLightAtDay PlayFromStart))))))
                        (:then_4
                          (goto _label_2 Reset))))))))))))))

(event EventBeginPlay
  (bind _sky_light (Variables|Sky|GetSky%20Light))
  (bind _sky_light_2 (Variables|Sky|GetSky%20Light))
  (bind _lightcomponent (Variables|/Script/Engine.SkyLight|GetLightComponent _sky_light))
  (bind _lightcomponent_2 (Variables|/Script/Engine.SkyLight|GetLightComponent _sky_light_2))
  (Utilities|FlowControl|Delay 0.2)
  (Utilities|FlowControl|Delay 0.2)
  (Utilities|IsValid (Variables|Sky|GetSky%20Light)
    (:Is%20Valid
      (if (< (Variables|Overridesettings|GetSun%20height) 0.0)
        ;[1 1 1] Night time
        (Rendering|Components|Light|SetIntensity _lightcomponent_2 (Variables|DayandNight|GetLightIntensityAtNight))
        (Class|SkyLightComponent|RecaptureSky _lightcomponent_2)
        (else
          ;[1 1 1] Day time
          (Rendering|Components|Light|SetIntensity _lightcomponent (Variables|DayandNight|GetLightIntensityAtDay))
          (Class|SkyLightComponent|RecaptureSky _lightcomponent))))))

(fn ConstructionScript
  (bind _moon_light_actor (Variables|Moon|GetMoon%20light%20actor))
  (bind _moon_light_actor_2 (Variables|Moon|GetMoon%20light%20actor))
  (bind _sun_light_actor (Variables|Sun|GetSun%20light%20actor))
  (bind _returnvalue (Transformation|GetActorRotation _moon_light_actor))
  (bind _lightcomponent (Variables|/Script/Engine.Light|GetLightComponent _moon_light_actor_2))
  (bind (_roll _pitch _yaw) (Math|Rotator|BreakRotator _returnvalue))
  (bind _returnvalue_2 (Rendering|Material|CreateDynamicMaterialInstance (Variables|BP_Skydome|GetSky%20Sphere%20mesh) 0 "/Game/CloudscapeSeasons/Materials/M_Sky.M_Sky" :!class /Script/Engine.PrimitiveComponent))
  (Variables|Sky|SetSky%20material _returnvalue_2)
  (if (Variables|Default|GetRefresh%20material) ; Updating bool in details panel causes construction script to run again
    _
    (else
      _))
  (Variables|Default|SetRefresh%20material false)
  (Utilities|FlowControl|Sequence
    (:then_0
      ;[1 1 1] Updates Sun Light Direction, Sun Color and Sun Height
      (Utilities|IsValid (Variables|Sun|GetSun%20light%20actor) ; Has a directional light been assigned?
        (:Is%20Valid
          (Rendering|Material|SetVectorParameterValue (Variables|Sky|GetSky%20material) "Sun color" (Math|Conversions|ToLinearColor(Color) (Variables|/Script/Engine.LightComponentBase|GetLightColor (Variables|/Script/Engine.Light|GetLightComponent _sun_light_actor))) :!class /Script/Engine.MaterialInstanceDynamic)
          (bind _output_get (Variables|Overridesettings|SetSun%20height (Math|Float|MapRangeUnclamped (.Pitch (Math|Rotator|BreakRotator (Transformation|GetActorRotation _sun_light_actor))) 0.0 -9e+01 0.0 1.0)))
          (Rendering|Material|SetScalarParameterValue (Variables|Sky|GetSky%20material) "Sun height" (Math|Float|SelectFloat (Math|Float|Absolute(Float) _output_get) 0.0 (< _output_get 0.0)) :!class /Script/Engine.MaterialInstanceDynamic)
          (Rendering|Material|SetVectorParameterValue (Variables|Sky|GetSky%20material) "SunLightVector" (Math|Conversions|ToLinearColor(Vector) (Math|Rotator|GetRotationXVector (Transformation|GetActorRotation _sun_light_actor))) :!class /Script/Engine.MaterialInstanceDynamic))))
    (:then_1
      ;[1 1 1] Updates Moon Light Direction and Moon Color
      (Utilities|IsValid _moon_light_actor ; Has a directional light been assigned?
        (:Is%20Valid
          (Rendering|Material|SetVectorParameterValue (Variables|Sky|GetSky%20material) "Moon color" (Math|Conversions|ToLinearColor(Color) (Variables|/Script/Engine.LightComponentBase|GetLightColor (Variables|/Script/Engine.Light|GetLightComponent _moon_light_actor))) :!class /Script/Engine.MaterialInstanceDynamic)
          (Rendering|Material|SetVectorParameterValue (Variables|Sky|GetSky%20material) "MoonLightVector" (Math|Conversions|ToLinearColor(Vector) (Math|Rotator|GetRotationXVector (Math|Rotator|MakeRotator _roll (* _pitch -1.0) _yaw))) :!class /Script/Engine.MaterialInstanceDynamic)
          (CallFunction|UpdateMoonShape))))
    (:then_2
      ;[1 1 1] Sets Sky Color with BP Parameters or from Curves if Colors Determined by Sun Position
      (if (Variables|Sun|GetColors%20determined%20by%20sun%20position)
        (Rendering|Material|SetVectorParameterValue (Variables|Sky|GetSky%20material) "Horizon color" (Math|Curves|GetLinearColorValue (Variables|Sky|GetHorizon%20color%20curve) (Variables|Overridesettings|GetSun%20height)) :!class /Script/Engine.MaterialInstanceDynamic)
        (Variables|Sky|SetHorizon%20color%20-%20current (Math|Curves|GetLinearColorValue (Variables|Sky|GetHorizon%20color%20curve) (Variables|Overridesettings|GetSun%20height)))
        (Rendering|Material|SetVectorParameterValue (Variables|Sky|GetSky%20material) "Zenith color" (Math|Curves|GetLinearColorValue (Variables|Sky|GetZenith%20color%20curve) (Variables|Overridesettings|GetSun%20height)) :!class /Script/Engine.MaterialInstanceDynamic)
        (Variables|Sky|SetZenith%20color%20-%20current (Math|Curves|GetLinearColorValue (Variables|Sky|GetZenith%20color%20curve) (Variables|Overridesettings|GetSun%20height)))
        (Rendering|Material|SetVectorParameterValue (Variables|Sky|GetSky%20material) "Cloud color" (Math|Curves|GetLinearColorValue (Variables|Sky|GetCloud%20color%20curve) (Variables|Overridesettings|GetSun%20height)) :!class /Script/Engine.MaterialInstanceDynamic)
        (Variables|Sky|SetCloud%20color%20-%20current (Math|Curves|GetLinearColorValue (Variables|Sky|GetCloud%20color%20curve) (Variables|Overridesettings|GetSun%20height)))
        (Rendering|Material|SetScalarParameterValue (Variables|Sky|GetSky%20material) "Horizon falloff" (Math|Float|Lerp 3.0 7.0 (Math|Float|Absolute(Float) (Variables|Overridesettings|GetSun%20height))) :!class /Script/Engine.MaterialInstanceDynamic)
        (else
          (Rendering|Material|SetVectorParameterValue (Variables|Sky|GetSky%20material) "Horizon color" (Variables|Overridesettings|GetHorizon%20color) :!class /Script/Engine.MaterialInstanceDynamic)
          (Rendering|Material|SetVectorParameterValue (Variables|Sky|GetSky%20material) "Zenith color" (Variables|Overridesettings|GetZenith%20Color) :!class /Script/Engine.MaterialInstanceDynamic)
          (Rendering|Material|SetVectorParameterValue (Variables|Sky|GetSky%20material) "Overall color" (Variables|Overridesettings|GetOverall%20Color) :!class /Script/Engine.MaterialInstanceDynamic)
          (Rendering|Material|SetVectorParameterValue (Variables|Sky|GetSky%20material) "Cloud color" (Variables|Overridesettings|GetCloud%20color) :!class /Script/Engine.MaterialInstanceDynamic)
          (Rendering|Material|SetScalarParameterValue (Variables|Sky|GetSky%20material) "Horizon falloff" (Variables|Overridesettings|GetHorizon%20Falloff) :!class /Script/Engine.MaterialInstanceDynamic))))
    (:then_3
      (Utilities|FlowControl|Sequence
        (:then_0
          ;[1 1 1] Clouds Parameters
          (Rendering|Material|SetScalarParameterValue (Variables|Sky|GetSky%20material) "Cloud speed" (Variables|Clouds|GetCloud%20speed) :!class /Script/Engine.MaterialInstanceDynamic)
          (Rendering|Material|SetScalarParameterValue (Variables|Sky|GetSky%20material) "Cloud opacity" (Variables|Clouds|GetCloud%20opacity) :!class /Script/Engine.MaterialInstanceDynamic)
          (if (Variables|Clouds|GetSimpleCloudsControl)
            (Rendering|Material|SetScalarParameterValue (Variables|Sky|GetSky%20material) "SimpleCloudsEnabled" 1.0 :!class /Script/Engine.MaterialInstanceDynamic)
            (else
              (Rendering|Material|SetScalarParameterValue (Variables|Sky|GetSky%20material) "SimpleCloudsEnabled" 0.0 :!class /Script/Engine.MaterialInstanceDynamic))))
        (:then_1
          ;[1 1 1] Sun Parameters
          (Utilities|IsValid (Variables|Sun|GetSun%20light%20actor)
            (:Is%20Valid
              (Rendering|Material|SetScalarParameterValue (Variables|Sky|GetSky%20material) "Sun brightness" (Variables|Sun|GetSun%20brightness) :!class /Script/Engine.MaterialInstanceDynamic)
              (Rendering|Material|SetScalarParameterValue (Variables|Sky|GetSky%20material) "Sun Radius" (Variables|Sun|GetSun%20Radius) :!class /Script/Engine.MaterialInstanceDynamic))))
        (:then_2
          ;[1 1 1] Stars Parameters
          (Rendering|Material|SetScalarParameterValue (Variables|Sky|GetSky%20material) "Stars brightness" (Variables|Stars|GetStars%20brightness) :!class /Script/Engine.MaterialInstanceDynamic)
          (Rendering|Material|SetScalarParameterValue (Variables|Sky|GetSky%20material) "Stars Amount" (Variables|Stars|GetStars%20amount) :!class /Script/Engine.MaterialInstanceDynamic)
          (Rendering|Material|SetScalarParameterValue (Variables|Sky|GetSky%20material) "StarsMovementSpeed" (Variables|Stars|GetStars%20movement%20speed) :!class /Script/Engine.MaterialInstanceDynamic))
        (:then_3
          ;[1 1 1] Moon Parameters
          (if (Variables|Moon|GetEnable%20Moon)
            (Utilities|IsValid _moon_light_actor_2 ; Has a directional light been assigned?
              (:Is%20Valid
                (Rendering|SetVisibility _lightcomponent (not (Utilities|Enum|Equal(Enum) (Variables|Moon|GetMoonPhase) "NewEnumerator0")) false)
                (Utilities|IsValid _moon_light_actor_2 ; Has a directional light been assigned?
                  (:Is%20Valid
                    (Rendering|Material|SetVectorParameterValue (Variables|Sky|GetSky%20material) "Moon color" (Math|Conversions|ToLinearColor(Color) (Variables|/Script/Engine.LightComponentBase|GetLightColor (Variables|/Script/Engine.Light|GetLightComponent _moon_light_actor_2))) :!class /Script/Engine.MaterialInstanceDynamic)
                    (Rendering|Material|SetScalarParameterValue (Variables|Sky|GetSky%20material) "Moon Radius" (Variables|Moon|GetMoon%20Radius) :!class /Script/Engine.MaterialInstanceDynamic)
                    (if (not (Utilities|Enum|Equal(Enum) (Variables|Moon|GetMoonPhase) "NewEnumerator0"))
                      (Rendering|Material|SetScalarParameterValue (Variables|Sky|GetSky%20material) "Moon Surface Contrast" (Variables|Moon|GetMoon%20Surface%20Contrast) :!class /Script/Engine.MaterialInstanceDynamic)
                      (else
                        (Rendering|Material|SetScalarParameterValue (Variables|Sky|GetSky%20material) "Moon Surface Contrast" 2.0 :!class /Script/Engine.MaterialInstanceDynamic)))))))
            (else
              (Utilities|IsValid _moon_light_actor_2 ; Has a directional light been assigned?
                (:Is%20Valid
                  (Rendering|SetVisibility _lightcomponent false false))))))))
    (:then_4
      (Networking|SetReplicates (Variables|Sky|GetSky%20Light) true))))

(fn UpdateSunDirection
  (bind _sun_light_actor (Variables|Sun|GetSun%20light%20actor))
  (bind _sky_material (Variables|Sky|GetSky%20material))
  (Utilities|IsValid (Variables|Sun|GetSun%20light%20actor)
    (:Is%20Valid
      (Variables|Overridesettings|SetSun%20height (Math|Float|MapRangeUnclamped (.Pitch (Math|Rotator|BreakRotator (Transformation|GetActorRotation _sun_light_actor))) 0.0 -9e+01 0.0 1.0))
      (Rendering|Material|SetVectorParameterValue _sky_material "SunLightVector" (Math|Conversions|ToLinearColor(Vector) (Math|Rotator|GetRotationXVector (Transformation|GetActorRotation _sun_light_actor))) :!class /Script/Engine.MaterialInstanceDynamic)
      (Rendering|Material|SetVectorParameterValue _sky_material "Sun color" (Math|Conversions|ToLinearColor(Color) (Variables|/Script/Engine.LightComponentBase|GetLightColor (Variables|/Script/Engine.Light|GetLightComponent (Variables|Sun|GetSun%20light%20actor)))) :!class /Script/Engine.MaterialInstanceDynamic)
      (Rendering|Material|SetScalarParameterValue _sky_material "Sun height" (Math|Float|SelectFloat (Math|Float|Absolute(Float) (Variables|Overridesettings|GetSun%20height)) 0.0 (< (Variables|Overridesettings|GetSun%20height) 0.0)) :!class /Script/Engine.MaterialInstanceDynamic)
      (if (Variables|Sun|GetColors%20determined%20by%20sun%20position)
        (Rendering|Material|SetVectorParameterValue _sky_material "Horizon color" (Math|Curves|GetLinearColorValue (Variables|Sky|GetHorizon%20color%20curve) (Variables|Overridesettings|GetSun%20height)) :!class /Script/Engine.MaterialInstanceDynamic)
        (Variables|Sky|SetHorizon%20color%20-%20current (Math|Curves|GetLinearColorValue (Variables|Sky|GetHorizon%20color%20curve) (Variables|Overridesettings|GetSun%20height)))
        (Rendering|Material|SetVectorParameterValue _sky_material "Zenith color" (Math|Curves|GetLinearColorValue (Variables|Sky|GetZenith%20color%20curve) (Variables|Overridesettings|GetSun%20height)) :!class /Script/Engine.MaterialInstanceDynamic)
        (Variables|Sky|SetZenith%20color%20-%20current (Math|Curves|GetLinearColorValue (Variables|Sky|GetZenith%20color%20curve) (Variables|Overridesettings|GetSun%20height)))
        (Rendering|Material|SetVectorParameterValue _sky_material "Cloud color" (Math|Curves|GetLinearColorValue (Variables|Sky|GetCloud%20color%20curve) (Variables|Overridesettings|GetSun%20height)) :!class /Script/Engine.MaterialInstanceDynamic)
        (Variables|Sky|SetCloud%20color%20-%20current (Math|Curves|GetLinearColorValue (Variables|Sky|GetCloud%20color%20curve) (Variables|Overridesettings|GetSun%20height)))
        (Rendering|Material|SetScalarParameterValue _sky_material "Horizon falloff" (Math|Float|Lerp 3.0 8.0 (Math|Float|Absolute(Float) (Variables|Overridesettings|GetSun%20height))) :!class /Script/Engine.MaterialInstanceDynamic)))))

(fn UpdateMoonDirection
  (bind _moon_light_actor (Variables|Moon|GetMoon%20light%20actor))
  (bind _sky_material (Variables|Sky|GetSky%20material))
  (bind _returnvalue (Transformation|GetActorRotation _moon_light_actor))
  (bind (_roll _pitch _yaw) (Math|Rotator|BreakRotator _returnvalue))
  (Utilities|IsValid (Variables|Moon|GetMoon%20light%20actor)
    (:Is%20Valid
      (Rendering|Material|SetVectorParameterValue _sky_material "MoonLightVector" (Math|Conversions|ToLinearColor(Vector) (Math|Rotator|GetRotationXVector (Math|Rotator|MakeRotator _roll (* _pitch -1.0) _yaw))) :!class /Script/Engine.MaterialInstanceDynamic)
      (Rendering|Material|SetVectorParameterValue _sky_material "Moon color" (Math|Conversions|ToLinearColor(Color) (Variables|/Script/Engine.LightComponentBase|GetLightColor (Variables|/Script/Engine.Light|GetLightComponent _moon_light_actor))) :!class /Script/Engine.MaterialInstanceDynamic)
      (CallFunction|UpdateMoonShape))))

(fn UpdateMoonShape
  (bind _sky_material (Variables|Sky|GetSky%20material))
  (bind _cloudscape_component (Variables|Clouds|GetCloudscape%20Component))
  (bind _cloudscape_component_2 (Variables|Clouds|GetCloudscape%20Component))
  (bind _moon (Variables|Moon|GetMoon))
  (if (Variables|Moon|GetEnable%20Moon%20Phase%20Transition)
    (Utilities|IsValid _moon
      (:Is%20Valid
        (bind _outrownames (DataTable|GetDataTableRowNames "/Game/CloudscapeSeasons/Blueprints/Assets/DT_MoonPhases.DT_MoonPhases"))
        (for _array_element _outrownames
          (bind _returnvalue (Utilities|GetDataTableRow "/Game/CloudscapeSeasons/Blueprints/Assets/DT_MoonPhases.DT_MoonPhases" _array_element)
            (:then
              (if (>= (Variables|/Game/CloudscapeSeasons/Blueprints/BP_TheMoon.BP_TheMoon_C|GetCurrentMoonPhase _moon) (.MoonPhaseApproxValue (Utilities|Struct|BreakSMoonPhases _returnvalue)))
                (Variables|Default|SetTmpMoonTexture (.MoonPicture (Utilities|Struct|BreakSMoonPhases _returnvalue)))
                (Variables|Default|SettmpMoonBrightness (.MoonPhaseBrightness (Utilities|Struct|BreakSMoonPhases _returnvalue)))
                (Utilities|IsValid _cloudscape_component
                  (:Is%20Valid
                    (if (Utilities|Enum|Equal(Enum) (.MoonPhase (Utilities|Struct|BreakSMoonPhases _returnvalue)) "NewEnumerator0")
                      (Variables|/Game/CloudscapeSeasons/Blueprints/BP_CloudscapeSeasons.BP_CloudscapeSeasons_C|SetIsNewMoon _cloudscape_component true)
                      (else
                        (Variables|/Game/CloudscapeSeasons/Blueprints/BP_CloudscapeSeasons.BP_CloudscapeSeasons_C|SetIsNewMoon _cloudscape_component false)))))))))))
    (else
      (bind _outrownames_2 (DataTable|GetDataTableRowNames "/Game/CloudscapeSeasons/Blueprints/Assets/DT_MoonPhases.DT_MoonPhases"))
      (for _array_element_2 _outrownames_2
        (bind _returnvalue_2 (Utilities|GetDataTableRow "/Game/CloudscapeSeasons/Blueprints/Assets/DT_MoonPhases.DT_MoonPhases" _array_element_2)
          (:then
            (if (Utilities|Enum|Equal(Enum) (.MoonPhase (Utilities|Struct|BreakSMoonPhases _returnvalue_2)) (Variables|Moon|GetMoonPhase))
              (Variables|Default|SetTmpMoonTexture (.MoonPicture (Utilities|Struct|BreakSMoonPhases _returnvalue_2)))
              (Variables|Default|SettmpMoonBrightness (.MoonPhaseBrightness (Utilities|Struct|BreakSMoonPhases _returnvalue_2)))
              (Utilities|IsValid _cloudscape_component_2
                (:Is%20Valid
                  (if (Utilities|Enum|Equal(Enum) (.MoonPhase (Utilities|Struct|BreakSMoonPhases _returnvalue_2)) "NewEnumerator0")
                    (Variables|/Game/CloudscapeSeasons/Blueprints/BP_CloudscapeSeasons.BP_CloudscapeSeasons_C|SetIsNewMoon _cloudscape_component_2 true)
                    (else
                      (Variables|/Game/CloudscapeSeasons/Blueprints/BP_CloudscapeSeasons.BP_CloudscapeSeasons_C|SetIsNewMoon _cloudscape_component_2 false)))))))))))
  (Rendering|Material|SetTextureParameterValue _sky_material "MoonTexture" (Variables|Default|GetTmpMoonTexture))
  (Rendering|Material|SetScalarParameterValue _sky_material "Moon brightness" (* (Variables|Default|GettmpMoonBrightness) (Variables|Moon|GetMoon%20brightness)) :!class /Script/Engine.MaterialInstanceDynamic))