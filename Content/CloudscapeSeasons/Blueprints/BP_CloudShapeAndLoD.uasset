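; Editor tool actor that bakes base cloud, detail and turbulence noise textures into render targets and previews them on labelled cubes.
; The construction script toggles and lays out the cubes in three rows.
; In DevelopmentMode it also creates dynamic materials and RGBA16f targets, draws the noise materials into them, then assigns per-channel and combined views to the cubes.
; The DevelopmentMode gate avoids an editor-load crash, and construction flags work around UE-42283.
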(event Custom|Bake
  (Utilities|FlowControl|Sequence
    (:then_0
      (Rendering|DrawMaterialtoRenderTarget (Variables|Blueprints&Materials|GetRT_BaseCloud) (Variables|Blueprints&Materials|GetM_BaseCloudInstance)))
    (:then_1
      (Rendering|DrawMaterialtoRenderTarget (Variables|Blueprints&Materials|GetRT_DetailsCloud) (Variables|Blueprints&Materials|GetM_DetailsCloudInstance)))
    (:then_2
      (Rendering|DrawMaterialtoRenderTarget (Variables|Blueprints&Materials|GetRT_Turbulence) (Variables|Blueprints&Materials|GetM_TurbCloudInstance)))))

(fn ConstructionScript
  (CallFunction|MainConstruct))

(fn MainConstruct
  (bind _result (CallFunction|GetTransformCorrected))
  (bind _result_2 (CallFunction|GetTransformCorrected))
  (bind _result_3 (CallFunction|GetTransformCorrected))
  (bind _rowseparationrelativetoboxesdistance (Variables|Default|GetRowSeparationRelativeToBoxesDistance))
  (bind _channeltextstartoffset (Variables|Default|GetChannelTextStartOffset))
  (bind _textstartoffset (Variables|Default|GetTextStartOffset))
  (bind _rowseparationrelativetoboxesdistance_2 (Variables|Default|GetRowSeparationRelativeToBoxesDistance))
  (bind _tool_boxes_distance (Variables|Default|GetTool%20Boxes%20Distance))
  (bind _tool_boxes_distance_2 (Variables|Default|GetTool%20Boxes%20Distance))
  (bind _visible (Variables|Default|GetVisible))
  (bind _textheightoffset (Variables|Default|GetTextHeightOffset))
  (bind (_location _rotation _scale) (Math|Transform|BreakTransform _result_3))
  (bind (_location_2 _rotation_2 _scale_2) (Math|Transform|BreakTransform _result_2))
  (bind (_location_3 _rotation_3 _scale_3) (Math|Transform|BreakTransform _result))
  (bind _returnvalue (* _tool_boxes_distance _rowseparationrelativetoboxesdistance))
  (bind _returnvalue_2 (* _tool_boxes_distance_2 _rowseparationrelativetoboxesdistance_2))
  (bind (_x _y _z) (Math|Vector|BreakVector _location))
  (bind (_x_2 _y_2 _z_2) (Math|Vector|BreakVector _location_2))
  (bind (_x_3 _y_3 _z_3) (Math|Vector|BreakVector _location_3))
  (bind _returnvalue_3 (+ _tool_boxes_distance _returnvalue))
  (bind _returnvalue_4 (+ _tool_boxes_distance_2 _returnvalue_2))
  (bind _returnvalue_5 (+ _z_2 _returnvalue_3))
  (bind _returnvalue_6 (* _returnvalue_4 2.0))
  (bind _returnvalue_7 (+ _z _returnvalue_6))
  ;[1 1 1] Needed to workaround issue UE-42283
  (if (Variables|WorkaroundUE-42283||GetConstructed)
    (Variables|WorkaroundUE-42283||Set1stConstructed false))
  ;[1 1 1] click on Update parameter to allow 1st construction of textures, which is prevented by issue UE-42283
  (if (Variables|Default|GetUpdate)
    (Variables|Default|SetUpdatePressed true)
    (else
      (Variables|Default|SetUpdatePressed false)))
  (Variables|Default|SetUpdate false)
  (Utilities|FlowControl|Sequence
    (:then_0
      ;[1 1 1] Enable/Disable Visibility for the tools if Development mode is active or not
      (Utilities|FlowControl|Sequence
        (:then_0
          (Rendering|SetVisibility (Variables|Default|GetRGBAHor01) _visible false))
        (:then_1
          ;;[1 1 1] transformation for Horizontal Layout
          (if _visible
            (bind _output_get (Variables|Default|SetYIncrement (Variables|Default|GetTool%20Boxes%20Distance)))
            (bind _output_get_2 (Variables|Default|SetXIncrement 0.0))
            (Transformation|SetWorldTransform (Variables|Default|GetCube3DText01R) (Math|Transform|MakeTransform (Math|Vector|MakeVector (+ _x_3 _output_get_2) (+ _y_3 (* _output_get 1.0)) _z_3) _rotation_3 _scale_3) false false)
            (Transformation|SetWorldTransform (Variables|Default|GetCube3DText01G) (Math|Transform|MakeTransform (Math|Vector|MakeVector (+ _x_3 _output_get_2) (+ _y_3 0.0) _z_3) _rotation_3 _scale_3) false false)
            (Transformation|SetWorldTransform (Variables|Default|GetCube3DText01B) (Math|Transform|MakeTransform (Math|Vector|MakeVector (+ _x_3 _output_get_2) (+ _y_3 (* _output_get -1.0)) _z_3) _rotation_3 _scale_3) false false)
            (Transformation|SetWorldTransform (Variables|Default|GetCube3DText01A) (Math|Transform|MakeTransform (Math|Vector|MakeVector (+ _x_3 _output_get_2) (+ _y_3 (* _output_get -2.0)) _z_3) _rotation_3 _scale_3) false false)
            (Transformation|SetWorldTransform (Variables|Default|GetCube3DText01Result) (Math|Transform|MakeTransform (Math|Vector|MakeVector (+ _x_3 _output_get_2) (+ _y_3 (* _output_get -3.0)) _z_3) _rotation_3 _scale_3) false false)
            (Transformation|SetWorldTransform (Variables|Default|GetCube3DText02R) (Math|Transform|MakeTransform (Math|Vector|MakeVector (+ _x_2 (Variables|Default|GetXIncrement)) (+ _y_2 (* (Variables|Default|GetYIncrement) 1.0)) _returnvalue_5) _rotation_2 _scale_2) false false)
            (Transformation|SetWorldTransform (Variables|Default|GetCube3DText02G) (Math|Transform|MakeTransform (Math|Vector|MakeVector (+ _x_2 (Variables|Default|GetXIncrement)) (+ _y_2 0.0) _returnvalue_5) _rotation _scale_2) false false)
            (Transformation|SetWorldTransform (Variables|Default|GetCube3DText02B) (Math|Transform|MakeTransform (Math|Vector|MakeVector (+ _x_2 (Variables|Default|GetXIncrement)) (+ _y_2 (* (Variables|Default|GetYIncrement) -1.0)) _returnvalue_5) _rotation_2 _scale_2) false false)
            (Transformation|SetWorldTransform (Variables|Default|GetCube3DText02Result) (Math|Transform|MakeTransform (Math|Vector|MakeVector (+ _x_2 (Variables|Default|GetXIncrement)) (+ _y_2 (* (Variables|Default|GetYIncrement) -2.0)) _returnvalue_5) _rotation_2 _scale_2) false false)
            (Transformation|SetWorldTransform (Variables|Default|GetCube2DText01R) (Math|Transform|MakeTransform (Math|Vector|MakeVector (+ _x (Variables|Default|GetXIncrement)) (+ _y (* (Variables|Default|GetYIncrement) 1.0)) _returnvalue_7) _rotation _scale) false false)
            (Transformation|SetWorldTransform (Variables|Default|GetCube2DText01G) (Math|Transform|MakeTransform (Math|Vector|MakeVector (+ _x (Variables|Default|GetXIncrement)) (+ _y 0.0) _returnvalue_7) _rotation _scale) false false)
            (Transformation|SetWorldTransform (Variables|Default|GetCube2DText01B) (Math|Transform|MakeTransform (Math|Vector|MakeVector (+ _x (Variables|Default|GetXIncrement)) (+ _y (* (Variables|Default|GetYIncrement) -1.0)) _returnvalue_7) _rotation _scale) false false)
            (Transformation|SetWorldTransform (Variables|Default|GetCube2DText01Result) (Math|Transform|MakeTransform (Math|Vector|MakeVector (+ _x (Variables|Default|GetXIncrement)) (+ _y (* (Variables|Default|GetYIncrement) -2.0)) _returnvalue_7) _rotation _scale) false false)
            (Transformation|SetWorldTransform (Variables|Default|GetRGBAHor01) (Math|Transform|MakeTransform (Math|Vector|MakeVector (.X (Math|Vector|BreakVector (.Location (Math|Transform|BreakTransform (Math|Transform|MakeTransform (Math|Vector|MakeVector (+ _x_3 _output_get_2) (+ _y_3 (* _output_get 1.0)) _z_3) _rotation_3 _scale_3))))) (+ (.Y (Math|Vector|BreakVector (.Location (Math|Transform|BreakTransform (Math|Transform|MakeTransform (Math|Vector|MakeVector (+ _x_3 _output_get_2) (+ _y_3 (* _output_get 1.0)) _z_3) _rotation_3 _scale_3))))) _channeltextstartoffset) (+ (.Z (Math|Vector|BreakVector (.Location (Math|Transform|BreakTransform (Math|Transform|MakeTransform (Math|Vector|MakeVector (+ _x_3 _output_get_2) (+ _y_3 (* _output_get 1.0)) _z_3) _rotation_3 _scale_3))))) (+ _textheightoffset 1e+01))) (.Rotation (Math|Transform|BreakTransform (Math|Transform|MakeTransform (Math|Vector|MakeVector (+ _x_3 _output_get_2) (+ _y_3 (* _output_get 1.0)) _z_3) _rotation_3 _scale_3))) (.Scale (Math|Transform|BreakTransform (Math|Transform|MakeTransform (Math|Vector|MakeVector (+ _x_3 _output_get_2) (+ _y_3 (* _output_get 1.0)) _z_3) _rotation_3 _scale_3)))) false false)
            (Transformation|SetWorldTransform (Variables|Default|GetRGBHor01) (Math|Transform|MakeTransform (Math|Vector|MakeVector (.X (Math|Vector|BreakVector (.Location (Math|Transform|BreakTransform (Math|Transform|MakeTransform (Math|Vector|MakeVector (+ _x_3 _output_get_2) (+ _y_3 (* _output_get 1.0)) _z_3) _rotation_3 _scale_3))))) (+ (.Y (Math|Vector|BreakVector (.Location (Math|Transform|BreakTransform (Math|Transform|MakeTransform (Math|Vector|MakeVector (+ _x_3 _output_get_2) (+ _y_3 (* _output_get 1.0)) _z_3) _rotation_3 _scale_3))))) _channeltextstartoffset) (+ (.Z (Math|Vector|BreakVector (.Location (Math|Transform|BreakTransform (Math|Transform|MakeTransform (Math|Vector|MakeVector (+ _x_3 _output_get_2) (+ _y_3 (* _output_get 1.0)) _z_3) _rotation_3 _scale_3))))) (+ _returnvalue_4 _textheightoffset))) (.Rotation (Math|Transform|BreakTransform (Math|Transform|MakeTransform (Math|Vector|MakeVector (+ _x_3 _output_get_2) (+ _y_3 (* _output_get 1.0)) _z_3) _rotation_3 _scale_3))) (.Scale (Math|Transform|BreakTransform (Math|Transform|MakeTransform (Math|Vector|MakeVector (+ _x_3 _output_get_2) (+ _y_3 (* _output_get 1.0)) _z_3) _rotation_3 _scale_3)))) false false)
            (Transformation|SetWorldTransform (Variables|Default|GetRGBHor02) (Math|Transform|MakeTransform (Math|Vector|MakeVector (.X (Math|Vector|BreakVector (.Location (Math|Transform|BreakTransform (Math|Transform|MakeTransform (Math|Vector|MakeVector (+ _x_3 _output_get_2) (+ _y_3 (* _output_get 1.0)) _z_3) _rotation_3 _scale_3))))) (+ (.Y (Math|Vector|BreakVector (.Location (Math|Transform|BreakTransform (Math|Transform|MakeTransform (Math|Vector|MakeVector (+ _x_3 _output_get_2) (+ _y_3 (* _output_get 1.0)) _z_3) _rotation_3 _scale_3))))) _channeltextstartoffset) (+ (.Z (Math|Vector|BreakVector (.Location (Math|Transform|BreakTransform (Math|Transform|MakeTransform (Math|Vector|MakeVector (+ _x_3 _output_get_2) (+ _y_3 (* _output_get 1.0)) _z_3) _rotation_3 _scale_3))))) (+ _returnvalue_6 _textheightoffset))) (.Rotation (Math|Transform|BreakTransform (Math|Transform|MakeTransform (Math|Vector|MakeVector (+ _x_3 _output_get_2) (+ _y_3 (* _output_get 1.0)) _z_3) _rotation_3 _scale_3))) (.Scale (Math|Transform|BreakTransform (Math|Transform|MakeTransform (Math|Vector|MakeVector (+ _x_3 _output_get_2) (+ _y_3 (* _output_get 1.0)) _z_3) _rotation_3 _scale_3)))) false false)
            (Transformation|SetWorldTransform (Variables|Default|GetCloudBaseNoise) (Math|Transform|MakeTransform (Math|Vector|MakeVector (.X (Math|Vector|BreakVector (.Location (Math|Transform|BreakTransform (Math|Transform|MakeTransform (Math|Vector|MakeVector (+ _x_3 _output_get_2) (+ _y_3 (* _output_get 1.0)) _z_3) _rotation_3 _scale_3))))) (+ (.Y (Math|Vector|BreakVector (.Location (Math|Transform|BreakTransform (Math|Transform|MakeTransform (Math|Vector|MakeVector (+ _x_3 _output_get_2) (+ _y_3 (* _output_get 1.0)) _z_3) _rotation_3 _scale_3))))) _textstartoffset) (+ (.Z (Math|Vector|BreakVector (.Location (Math|Transform|BreakTransform (Math|Transform|MakeTransform (Math|Vector|MakeVector (+ _x_3 _output_get_2) (+ _y_3 (* _output_get 1.0)) _z_3) _rotation_3 _scale_3))))) 0.0)) (.Rotation (Math|Transform|BreakTransform (Math|Transform|MakeTransform (Math|Vector|MakeVector (+ _x_3 _output_get_2) (+ _y_3 (* _output_get 1.0)) _z_3) _rotation_3 _scale_3))) (.Scale (Math|Transform|BreakTransform (Math|Transform|MakeTransform (Math|Vector|MakeVector (+ _x_3 _output_get_2) (+ _y_3 (* _output_get 1.0)) _z_3) _rotation_3 _scale_3)))) false false)
            (Transformation|SetWorldTransform (Variables|Default|GetCloudDetailNoise) (Math|Transform|MakeTransform (Math|Vector|MakeVector (.X (Math|Vector|BreakVector (.Location (Math|Transform|BreakTransform (Math|Transform|MakeTransform (Math|Vector|MakeVector (+ _x_3 _output_get_2) (+ _y_3 (* _output_get 1.0)) _z_3) _rotation_3 _scale_3))))) (+ (.Y (Math|Vector|BreakVector (.Location (Math|Transform|BreakTransform (Math|Transform|MakeTransform (Math|Vector|MakeVector (+ _x_3 _output_get_2) (+ _y_3 (* _output_get 1.0)) _z_3) _rotation_3 _scale_3))))) _textstartoffset) (+ (.Z (Math|Vector|BreakVector (.Location (Math|Transform|BreakTransform (Math|Transform|MakeTransform (Math|Vector|MakeVector (+ _x_3 _output_get_2) (+ _y_3 (* _output_get 1.0)) _z_3) _rotation_3 _scale_3))))) _returnvalue_4)) (.Rotation (Math|Transform|BreakTransform (Math|Transform|MakeTransform (Math|Vector|MakeVector (+ _x_3 _output_get_2) (+ _y_3 (* _output_get 1.0)) _z_3) _rotation_3 _scale_3))) (.Scale (Math|Transform|BreakTransform (Math|Transform|MakeTransform (Math|Vector|MakeVector (+ _x_3 _output_get_2) (+ _y_3 (* _output_get 1.0)) _z_3) _rotation_3 _scale_3)))) false false)
            (Transformation|SetWorldTransform (Variables|Default|GetCurlNoise) (Math|Transform|MakeTransform (Math|Vector|MakeVector (.X (Math|Vector|BreakVector (.Location (Math|Transform|BreakTransform (Math|Transform|MakeTransform (Math|Vector|MakeVector (+ _x_3 _output_get_2) (+ _y_3 (* _output_get 1.0)) _z_3) _rotation_3 _scale_3))))) (+ (.Y (Math|Vector|BreakVector (.Location (Math|Transform|BreakTransform (Math|Transform|MakeTransform (Math|Vector|MakeVector (+ _x_3 _output_get_2) (+ _y_3 (* _output_get 1.0)) _z_3) _rotation_3 _scale_3))))) _textstartoffset) (+ (.Z (Math|Vector|BreakVector (.Location (Math|Transform|BreakTransform (Math|Transform|MakeTransform (Math|Vector|MakeVector (+ _x_3 _output_get_2) (+ _y_3 (* _output_get 1.0)) _z_3) _rotation_3 _scale_3))))) _returnvalue_6)) (.Rotation (Math|Transform|BreakTransform (Math|Transform|MakeTransform (Math|Vector|MakeVector (+ _x_3 _output_get_2) (+ _y_3 (* _output_get 1.0)) _z_3) _rotation_3 _scale_3))) (.Scale (Math|Transform|BreakTransform (Math|Transform|MakeTransform (Math|Vector|MakeVector (+ _x_3 _output_get_2) (+ _y_3 (* _output_get 1.0)) _z_3) _rotation_3 _scale_3)))) false false)))))
    (:then_1
      ;[1 1 1] This fixes crash during the editor load with the default editor map containing a level which has an instance of this blueprint
      (if (Variables|Default|GetDevelopmentMode)
        (Utilities|FlowControl|Sequence
          (:then_0
            (CallFunction|CreateDynamicMaterials))
          (:then_1
            (CallFunction|CreateRenderTargets)
            (CallFunction|Bake))
          (:then_2
            (CallFunction|SetDynamicMaterials))
          (:then_3
            (CallFunction|SetupCubes))
          (:then_4
            (Variables|Default|SetUpdatePressed false)
            (Variables|WorkaroundUE-42283||SetConstructed true)))))))

(fn CreateDynamicMaterials
  (bind _lod_cube_one_channel_mat (Variables|Blueprints&Materials|GetLoD%20Cube%20One%20Channel%20Mat))
  (bind _lod_cube_three_channel_mat (Variables|Blueprints&Materials|GetLoD%20Cube%20Three%20Channel%20Mat))
  (bind _details_cloud_material (Variables|Blueprints&Materials|GetDetails%20Cloud%20Material))
  (bind _turbulence_cloud_material (Variables|Blueprints&Materials|GetTurbulence%20Cloud%20Material))
  (bind _lod_cube_three_channel_color_mat (Variables|Blueprints&Materials|GetLoD%20Cube%20Three%20Channel%20Color%20Mat))
  (bind _lod_cube_four_channel_mat (Variables|Blueprints&Materials|GetLoD%20Cube%20Four%20Channel%20Mat))
  (bind _base_cloud_material (Variables|Blueprints&Materials|GetBase%20Cloud%20Material))
  (Utilities|FlowControl|Sequence
    (:then_0
      ;[1 1 1] Base Cloud Material Dyn Instance
      (Utilities|IsValid _base_cloud_material
        (:Is%20Valid
          (bind _returnvalue (Rendering|Material|CreateDynamicMaterialInstance _base_cloud_material "None" :!class /Script/Engine.KismetMaterialLibrary))
          (Variables|Blueprints&Materials|SetM_BaseCloudInstance _returnvalue))))
    (:then_1
      ;[1 1 1] Details Cloud Material Dyn Instance
      (Utilities|IsValid _details_cloud_material
        (:Is%20Valid
          (bind _returnvalue_2 (Rendering|Material|CreateDynamicMaterialInstance _details_cloud_material "None" :!class /Script/Engine.KismetMaterialLibrary))
          (Variables|Blueprints&Materials|SetM_DetailsCloudInstance _returnvalue_2))))
    (:then_2
      ;[1 1 1] Turbulence Material Dyn Instance
      (Utilities|IsValid _turbulence_cloud_material
        (:Is%20Valid
          (bind _returnvalue_3 (Rendering|Material|CreateDynamicMaterialInstance _turbulence_cloud_material "None" :!class /Script/Engine.KismetMaterialLibrary))
          (Variables|Blueprints&Materials|SetM_TurbCloudInstance _returnvalue_3))))
    (:then_3
      ;[1 1 1] LoD Cube One Channel Mat Dyn Instance
      (Utilities|IsValid _lod_cube_one_channel_mat
        (:Is%20Valid
          (bind _returnvalue_4 (Rendering|Material|CreateDynamicMaterialInstance _lod_cube_one_channel_mat "None" :!class /Script/Engine.KismetMaterialLibrary))
          (Variables|Blueprints&Materials|SetLoD%20Cube%20One%20Channel%203D01R%20Mat%20Instance _returnvalue_4)
          (bind _returnvalue_5 (Rendering|Material|CreateDynamicMaterialInstance _lod_cube_one_channel_mat "None" :!class /Script/Engine.KismetMaterialLibrary))
          (Variables|Blueprints&Materials|SetLoD%20Cube%20One%20Channel%203D01G%20Mat%20Instance _returnvalue_5)
          (bind _returnvalue_6 (Rendering|Material|CreateDynamicMaterialInstance _lod_cube_one_channel_mat "None" :!class /Script/Engine.KismetMaterialLibrary))
          (Variables|Blueprints&Materials|SetLoD%20Cube%20One%20Channel%203D01B%20Mat%20Instance _returnvalue_6)
          (bind _returnvalue_7 (Rendering|Material|CreateDynamicMaterialInstance _lod_cube_one_channel_mat "None" :!class /Script/Engine.KismetMaterialLibrary))
          (Variables|Blueprints&Materials|SetLoD%20Cube%20One%20Channel%203D01A%20Mat%20Instance _returnvalue_7)
          (bind _returnvalue_8 (Rendering|Material|CreateDynamicMaterialInstance _lod_cube_one_channel_mat "None" :!class /Script/Engine.KismetMaterialLibrary))
          (Variables|Blueprints&Materials|SetLoD%20Cube%20One%20Channel%203D02R%20Mat%20Instance _returnvalue_8)
          (bind _returnvalue_9 (Rendering|Material|CreateDynamicMaterialInstance _lod_cube_one_channel_mat "None" :!class /Script/Engine.KismetMaterialLibrary))
          (Variables|Blueprints&Materials|SetLoD%20Cube%20One%20Channel%203D02G%20Mat%20Instance _returnvalue_9)
          (bind _returnvalue_10 (Rendering|Material|CreateDynamicMaterialInstance _lod_cube_one_channel_mat "None" :!class /Script/Engine.KismetMaterialLibrary))
          (Variables|Blueprints&Materials|SetLoD%20Cube%20One%20Channel%203D02B%20Mat%20Instance _returnvalue_10)
          (bind _returnvalue_11 (Rendering|Material|CreateDynamicMaterialInstance _lod_cube_one_channel_mat "None" :!class /Script/Engine.KismetMaterialLibrary))
          (Variables|Blueprints&Materials|SetLoD%20Cube%20One%20Channel%202D01R%20Mat%20Instance _returnvalue_11)
          (bind _returnvalue_12 (Rendering|Material|CreateDynamicMaterialInstance _lod_cube_one_channel_mat "None" :!class /Script/Engine.KismetMaterialLibrary))
          (Variables|Blueprints&Materials|SetLoD%20Cube%20One%20Channel%202D01G%20Mat%20Instance _returnvalue_12)
          (bind _returnvalue_13 (Rendering|Material|CreateDynamicMaterialInstance _lod_cube_one_channel_mat "None" :!class /Script/Engine.KismetMaterialLibrary))
          (Variables|Blueprints&Materials|SetLoD%20Cube%20One%20Channel%202D01B%20Mat%20Instance _returnvalue_13))))
    (:then_4
      ;[1 1 1] LoD Cube Three Channel Mat Dyn Instance
      (Utilities|IsValid _lod_cube_three_channel_mat
        (:Is%20Valid
          (bind _returnvalue_14 (Rendering|Material|CreateDynamicMaterialInstance _lod_cube_three_channel_mat "None" :!class /Script/Engine.KismetMaterialLibrary))
          (Variables|Blueprints&Materials|SetLoD%20Cube%20Three%20Channel%20Mat%20Instance _returnvalue_14))))
    (:then_5
      ;[1 1 1] LoD Cube Three Channel Color Mat Dyn Instance
      (Utilities|IsValid _lod_cube_three_channel_color_mat
        (:Is%20Valid
          (bind _returnvalue_15 (Rendering|Material|CreateDynamicMaterialInstance _lod_cube_three_channel_color_mat "None" :!class /Script/Engine.KismetMaterialLibrary))
          (Variables|Blueprints&Materials|SetLoD%20Cube%20Three%20Channel%20Color%20Mat%20Instance _returnvalue_15))))
    (:then_6
      ;[1 1 1] LoD Cube Four Channel Mat Dyn Instance
      (Utilities|IsValid _lod_cube_four_channel_mat
        (:Is%20Valid
          (bind _returnvalue_16 (Rendering|Material|CreateDynamicMaterialInstance _lod_cube_four_channel_mat "None" :!class /Script/Engine.KismetMaterialLibrary))
          (Variables|Blueprints&Materials|SetLoD%20Cube%20Four%20Channel%20Mat%20Instance _returnvalue_16))))))

(fn SetDynamicMaterials
  (bind _rt_basecloud (Variables|Blueprints&Materials|GetRT_BaseCloud))
  (bind _rt_detailscloud (Variables|Blueprints&Materials|GetRT_DetailsCloud))
  (bind _rt_turbulence (Variables|Blueprints&Materials|GetRT_Turbulence))
  (Utilities|FlowControl|Sequence
    (:then_0
      (Rendering|Material|SetTextureParameterValue (Variables|Blueprints&Materials|GetLoD%20Cube%20One%20Channel%203D01R%20Mat%20Instance) "Texture" _rt_basecloud)
      (Rendering|Material|SetTextureParameterValue (Variables|Blueprints&Materials|GetLoD%20Cube%20One%20Channel%203D01G%20Mat%20Instance) "Texture" _rt_basecloud)
      (Rendering|Material|SetTextureParameterValue (Variables|Blueprints&Materials|GetLoD%20Cube%20One%20Channel%203D01B%20Mat%20Instance) "Texture" _rt_basecloud)
      (Rendering|Material|SetTextureParameterValue (Variables|Blueprints&Materials|GetLoD%20Cube%20One%20Channel%203D01A%20Mat%20Instance) "Texture" _rt_basecloud)
      (Rendering|Material|SetTextureParameterValue (Variables|Blueprints&Materials|GetLoD%20Cube%20One%20Channel%203D02R%20Mat%20Instance) "Texture" _rt_detailscloud)
      (Rendering|Material|SetTextureParameterValue (Variables|Blueprints&Materials|GetLoD%20Cube%20One%20Channel%203D02G%20Mat%20Instance) "Texture" _rt_detailscloud)
      (Rendering|Material|SetTextureParameterValue (Variables|Blueprints&Materials|GetLoD%20Cube%20One%20Channel%203D02B%20Mat%20Instance) "Texture" _rt_detailscloud)
      (Rendering|Material|SetTextureParameterValue (Variables|Blueprints&Materials|GetLoD%20Cube%20One%20Channel%202D01R%20Mat%20Instance) "Texture" _rt_turbulence)
      (Rendering|Material|SetTextureParameterValue (Variables|Blueprints&Materials|GetLoD%20Cube%20One%20Channel%202D01G%20Mat%20Instance) "Texture" _rt_turbulence)
      (Rendering|Material|SetTextureParameterValue (Variables|Blueprints&Materials|GetLoD%20Cube%20One%20Channel%202D01B%20Mat%20Instance) "Texture" _rt_turbulence)
      (Rendering|Material|SetVectorParameterValue (Variables|Blueprints&Materials|GetLoD%20Cube%20One%20Channel%203D01R%20Mat%20Instance) "Channel" (Utilities|Struct|MakeLinearColor 1.0 0.0 0.0 0.0) :!class /Script/Engine.MaterialInstanceDynamic)
      (Rendering|Material|SetVectorParameterValue (Variables|Blueprints&Materials|GetLoD%20Cube%20One%20Channel%203D01G%20Mat%20Instance) "Channel" (Utilities|Struct|MakeLinearColor 0.0 1.0 0.0 0.0) :!class /Script/Engine.MaterialInstanceDynamic)
      (Rendering|Material|SetVectorParameterValue (Variables|Blueprints&Materials|GetLoD%20Cube%20One%20Channel%203D01B%20Mat%20Instance) "Channel" (Utilities|Struct|MakeLinearColor 0.0 0.0 1.0 0.0) :!class /Script/Engine.MaterialInstanceDynamic)
      (Rendering|Material|SetVectorParameterValue (Variables|Blueprints&Materials|GetLoD%20Cube%20One%20Channel%203D01A%20Mat%20Instance) "Channel" (Utilities|Struct|MakeLinearColor 0.0 0.0 0.0 1.0) :!class /Script/Engine.MaterialInstanceDynamic))
    (:then_1
      (Rendering|Material|SetTextureParameterValue (Variables|Blueprints&Materials|GetLoD%20Cube%20Three%20Channel%20Mat%20Instance) "Texture" (Variables|Blueprints&Materials|GetRT_DetailsCloud)))
    (:then_2
      (Rendering|Material|SetTextureParameterValue (Variables|Blueprints&Materials|GetLoD%20Cube%20Three%20Channel%20Color%20Mat%20Instance) "Texture" (Variables|Blueprints&Materials|GetRT_Turbulence)))
    (:then_3
      (Rendering|Material|SetTextureParameterValue (Variables|Blueprints&Materials|GetLoD%20Cube%20Four%20Channel%20Mat%20Instance) "Texture" (Variables|Blueprints&Materials|GetRT_BaseCloud)))))

(fn SetupCubes
  (Rendering|Material|SetMaterial (Variables|Default|GetCube3DText01R) 0 (Variables|Blueprints&Materials|GetLoD%20Cube%20One%20Channel%203D01R%20Mat%20Instance))
  (Rendering|Material|SetMaterial (Variables|Default|GetCube3DText02R) 0 (Variables|Blueprints&Materials|GetLoD%20Cube%20One%20Channel%203D02R%20Mat%20Instance))
  (Rendering|Material|SetMaterial (Variables|Default|GetCube2DText01R) 0 (Variables|Blueprints&Materials|GetLoD%20Cube%20One%20Channel%202D01R%20Mat%20Instance))
  (Rendering|Material|SetMaterial (Variables|Default|GetCube3DText01G) 0 (Variables|Blueprints&Materials|GetLoD%20Cube%20One%20Channel%203D01G%20Mat%20Instance))
  (Rendering|Material|SetMaterial (Variables|Default|GetCube3DText02G) 0 (Variables|Blueprints&Materials|GetLoD%20Cube%20One%20Channel%203D02G%20Mat%20Instance))
  (Rendering|Material|SetMaterial (Variables|Default|GetCube2DText01G) 0 (Variables|Blueprints&Materials|GetLoD%20Cube%20One%20Channel%202D01G%20Mat%20Instance))
  (Rendering|Material|SetMaterial (Variables|Default|GetCube3DText01B) 0 (Variables|Blueprints&Materials|GetLoD%20Cube%20One%20Channel%203D01B%20Mat%20Instance))
  (Rendering|Material|SetMaterial (Variables|Default|GetCube3DText02B) 0 (Variables|Blueprints&Materials|GetLoD%20Cube%20One%20Channel%203D02B%20Mat%20Instance))
  (Rendering|Material|SetMaterial (Variables|Default|GetCube2DText01B) 0 (Variables|Blueprints&Materials|GetLoD%20Cube%20One%20Channel%202D01B%20Mat%20Instance))
  (Rendering|Material|SetMaterial (Variables|Default|GetCube3DText01A) 0 (Variables|Blueprints&Materials|GetLoD%20Cube%20One%20Channel%203D01A%20Mat%20Instance))
  (Rendering|Material|SetMaterial (Variables|Default|GetCube3DText01Result) 0 (Variables|Blueprints&Materials|GetLoD%20Cube%20Four%20Channel%20Mat%20Instance))
  (Rendering|Material|SetMaterial (Variables|Default|GetCube3DText02Result) 0 (Variables|Blueprints&Materials|GetLoD%20Cube%20Three%20Channel%20Mat%20Instance))
  (Rendering|Material|SetMaterial (Variables|Default|GetCube2DText01Result) 0 (Variables|Blueprints&Materials|GetLoD%20Cube%20Three%20Channel%20Color%20Mat%20Instance)))

(fn CreateRenderTargets
  (bind _base_cloud_texture_size (Variables|Blueprints&Materials|GetBase%20Cloud%20Texture%20Size))
  (bind _details_cloud_texture_size (Variables|Blueprints&Materials|GetDetails%20Cloud%20Texture%20Size))
  (bind _turbulence_cloud_texture_size (Variables|Blueprints&Materials|GetTurbulence%20Cloud%20Texture%20Size))
  (Utilities|FlowControl|Sequence
    (:then_0
      (bind _returnvalue (Rendering|CreateRenderTarget2D _base_cloud_texture_size _base_cloud_texture_size "RTF_RGBA16f"))
      (Variables|Blueprints&Materials|SetRT_BaseCloud _returnvalue))
    (:then_1
      (bind _returnvalue_2 (Rendering|CreateRenderTarget2D _details_cloud_texture_size _details_cloud_texture_size "RTF_RGBA16f"))
      (Variables|Blueprints&Materials|SetRT_DetailsCloud _returnvalue_2))
    (:then_2
      (bind _returnvalue_3 (Rendering|CreateRenderTarget2D _turbulence_cloud_texture_size _turbulence_cloud_texture_size "RTF_RGBA16f"))
      (Variables|Blueprints&Materials|SetRT_Turbulence _returnvalue_3))))

(fn GetTransformCorrected
  (bind _billboard (Variables|Components|GetBillboard))
  (bind _returnvalue (Transformation|GetWorldTransform _billboard))
  (bind (_location _rotation _scale) (Math|Transform|BreakTransform _returnvalue))
  (bind (_x _y _z) (Math|Vector|BreakVector _location))
  (return (Math|Transform|MakeTransform (Math|Vector|MakeVector (- _x 9e+02) (- _y 3e+02) (+ _z 2e+02)) _rotation (* _scale 1.5))))