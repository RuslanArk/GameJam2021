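; BP_BakeTexture is a utility actor in CloudscapeSeasons that bakes a material into a render target texture.
; Its construction script resets the Bake flag and calls BakeIt whenever MaterialToBake is valid, regardless of the flag's value.
; BakeIt checks the render target, clears it to opaque black and draws the material into it.
; BeginPlay, overlap and Tick do nothing, so baking is driven by construction alone.
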(event Custom|BakeIt
  (bind _rendertarget (Variables|Default|GetRenderTarget))
  (Utilities|IsValid (Variables|Default|GetRenderTarget)
    (:Is%20Valid
      (Rendering|ClearRenderTarget2D _rendertarget)
      (Rendering|DrawMaterialtoRenderTarget _rendertarget (Variables|Default|GetMaterialToBake)))))

(event EventBeginPlay)

(event Collision|EventActorBeginOverlap
  (params (OtherActor :type Actor%20Object%20Reference)))

(event EventTick
  (params (DeltaSeconds :type Float%20%28single-precision%29)))

(fn ConstructionScript
  (if (Variables|Default|GetBake)
    _
    (else
      _))
  (Variables|Default|SetBake false)
  (Utilities|IsValid (Variables|Default|GetMaterialToBake)
    (:Is%20Valid
      (CallFunction|BakeIt))))