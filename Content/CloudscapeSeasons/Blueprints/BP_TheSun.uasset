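; Sun actor that rotates a movable directional Sunlight to follow the date, time and location held by a Calendar.
; Construction, BeginPlay and an interval-throttled Tick (when Enabled) copy Calendar values, then update the trajectory.
; The Calendar's TimeEvolution selects an astronomical path, a simplified circular path mapped from time of day, or a stored rotation.
; The astronomical path derives elevation and azimuth from latitude, longitude, equation of time, declination and hour angle.
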(event EventBeginPlay
  (CallFunction|UpdateDateTime)
  (CallFunction|UpdateTrajectory))

(event EventTick
  (params (DeltaSeconds :type Float%20%28single-precision%29))
  (if (Variables|Default|GetEnabled)
    (bind _output_get (Variables|Default|SetLastUpdate (+ DeltaSeconds (Variables|Default|GetLastUpdate))))
    (if (>= _output_get (Variables|Default|GetTrajectoryUpdateInterval))
      (Variables|Default|SetLastUpdate 0.0)
      (CallFunction|UpdateDateTime)
      (CallFunction|UpdateTrajectory))))

(fn ConstructionScript
  (if (Variables|Default|GetRefresh)
    _
    (else
      _))
  (Variables|Default|SetRefresh false)
  (CallFunction|UpdateDateTime)
  (CallFunction|UpdateTrajectory))

(fn UpdateTrajectory
  (bind _sunlight (Variables|Default|GetSunlight))
  (bind _calendar (Variables|Default|GetCalendar))
  (bind _time_evolution (Variables|/Game/CloudscapeSeasons/Blueprints/BP_CalendarSeasons.BP_CalendarSeasons_C|GetTime%20Evolution _calendar))
  (Utilities|IsValid _sunlight
    (:Is%20Valid
      (if (Utilities|Enum|Equal(Enum) (Variables|/Script/Engine.SceneComponent|GetMobility (Variables|/Script/Engine.Light|GetLightComponent _sunlight)) "Movable")
        (Utilities|IsValid _calendar
          (:Is%20Valid
            (if (Utilities|Enum|Equal(Enum) _time_evolution "NewEnumerator0")
              ;[1 1 1] Longitude/Latitude Based Trajectory
              (Transformation|SetWorldRotation (Variables|/Script/Engine.Light|GetLightComponent (Variables|Default|GetSunlight)) (CallFunction|CalculateTrajectory (Variables|Default|GetLatitude) (Variables|Default|GetLongitude) (Variables|Default|GetHour) (Variables|Default|GetMinute) (Variables|Default|GetSecond) (Variables|Default|GetYear) (Variables|Default|GetMonth) (Variables|Default|GetDay) (Variables|Default|GetDST)) false false)
              (elif (Utilities|Enum|Equal(Enum) _time_evolution "NewEnumerator1")
                ;[1 1 1] Circular Based Trajectory
                (Transformation|SetWorldRotation (Variables|/Script/Engine.Light|GetLightComponent (Variables|Default|GetSunlight)) (CallFunction|CalculateTrajectoryCircular (Variables|Default|GetHour) (Variables|Default|GetMinute) (Variables|Default|GetSecond)) false false)
                (elif (Utilities|Enum|Equal(Enum) _time_evolution "NewEnumerator2")
                  (Transformation|SetWorldRotation (Variables|/Script/Engine.Light|GetLightComponent (Variables|Default|GetSunlight)) (Variables|Default|GetRotator) false false))))))))))

(fn UpdateDateTime
  (bind _calendar (Variables|Default|GetCalendar))
  (Utilities|IsValid _calendar
    (:Is%20Valid
      (Variables|Default|SetDST (Variables|/Game/CloudscapeSeasons/Blueprints/BP_CalendarSeasons.BP_CalendarSeasons_C|GetDST _calendar))
      (Variables|Default|SetLatitude%20Degrees (Variables|/Game/CloudscapeSeasons/Blueprints/BP_CalendarSeasons.BP_CalendarSeasons_C|GetLatitude%20Degrees _calendar))
      (Variables|Default|SetLatitude%20Minutes (Variables|/Game/CloudscapeSeasons/Blueprints/BP_CalendarSeasons.BP_CalendarSeasons_C|GetLatitude%20Minutes _calendar))
      (Variables|Default|SetLatitude%20Seconds (Variables|/Game/CloudscapeSeasons/Blueprints/BP_CalendarSeasons.BP_CalendarSeasons_C|GetLatitude%20Seconds _calendar))
      (Variables|Default|SetLongitude%20Degrees (Variables|/Game/CloudscapeSeasons/Blueprints/BP_CalendarSeasons.BP_CalendarSeasons_C|GetLongitude%20Degrees _calendar))
      (Variables|Default|SetLongitude%20Minutes (Variables|/Game/CloudscapeSeasons/Blueprints/BP_CalendarSeasons.BP_CalendarSeasons_C|GetLongitude%20Minutes _calendar))
      (Variables|Default|SetLongitude%20Seconds (Variables|/Game/CloudscapeSeasons/Blueprints/BP_CalendarSeasons.BP_CalendarSeasons_C|GetLongitude%20Seconds _calendar))
      (Variables|Default|SetLatitude (Variables|/Game/CloudscapeSeasons/Blueprints/BP_CalendarSeasons.BP_CalendarSeasons_C|GetLatitude _calendar))
      (Variables|Default|SetLongitude (Variables|/Game/CloudscapeSeasons/Blueprints/BP_CalendarSeasons.BP_CalendarSeasons_C|GetLongitude _calendar))
      (Variables|Default|SetYear (Variables|/Game/CloudscapeSeasons/Blueprints/BP_CalendarSeasons.BP_CalendarSeasons_C|GetYear _calendar))
      (Variables|Default|SetMonth (Variables|/Game/CloudscapeSeasons/Blueprints/BP_CalendarSeasons.BP_CalendarSeasons_C|GetMonth _calendar))
      (Variables|Default|SetDay (Variables|/Game/CloudscapeSeasons/Blueprints/BP_CalendarSeasons.BP_CalendarSeasons_C|GetDay _calendar))
      (Variables|Default|SetHour (Variables|/Game/CloudscapeSeasons/Blueprints/BP_CalendarSeasons.BP_CalendarSeasons_C|GetHour _calendar))
      (Variables|Default|SetMinute (Variables|/Game/CloudscapeSeasons/Blueprints/BP_CalendarSeasons.BP_CalendarSeasons_C|GetMinutes _calendar))
      (Variables|Default|SetSecond (Variables|/Game/CloudscapeSeasons/Blueprints/BP_CalendarSeasons.BP_CalendarSeasons_C|GetSeconds _calendar)))))

(fn CalculateTrajectory
  (params (Latitude :type Float%20%28single-precision%29) (Longitude :type Float%20%28single-precision%29) (Hour :type Integer) (Minute :type Integer) (Second :type Integer) (Year :type Integer) (Month :type Integer) (Day :type Integer) (DST :type Boolean))
  (Utilities|FlowControl|Sequence
    (:then_0
      ;[1 1 1] Step 1
      (Variables|Default|Setdate (Math|DateTime|MakeDateTime Year Month Day Hour Minute Second)))
    (:then_1
      ;[1 1 1] Step 2
      (Variables|Default|SetDayOfYear (Math|Conversions|ToFloat(Integer) (- (Class|KismetMathLibrary|GetDayOfYear (Variables|Default|Getdate)) 1))))
    (:then_2
      ;[1 1 1] Step 3
      (Variables|Default|SetOffsetUTC 0.0)
      (if (Variables|Default|GetDST)
        (bind _result (Math|Float|IncrementFloat (Variables|Default|GetOffsetUTC))
          (:%20%20
            (Variables|Default|SetOffsetUTC _result)))))
    (:then_3
      ;[1 1 1] Step 4
      (Variables|Default|SetLSTM (* (Variables|Default|GetOffsetUTC) 15.0))
      (if (Variables|Default|GetDST)
        (Math|Float|DecrementFloat (Variables|Default|GetLSTM))))
    (:then_4
      ;[1 1 1] Step 5
      (Variables|Default|SetLct (Math|Timespan|GetTotalHours (TimeOfDay|GetTimeOfDay (Variables|Default|Getdate) :!class /Script/Engine.KismetMathLibrary))))
    (:then_5
      ;[1 1 1] Step 6
      (Variables|Default|SetEotBase (|(({DE2DE248-49E9-199D-EFBD-C0972F14DAD7}-81.000000)*(360.000000/365.242004)))))
    (:then_6
      ;[1 1 1] Step 7
      (Variables|Default|SetEot (|(((9.870000*(SINd(({786F2E82-4F43-F515-42AE-A3AF45F876E8}*2.000000))))-(7.530000*(COSd({786F2E82-4F43-F515-42AE-A3AF45F876E8}))))-(1.500000*(SINd({786F2E82-4F43-F515-42AE-A3AF45F876E8})))))))
    (:then_7
      ;[1 1 1] Step 8
      (Variables|Default|SetTcf (|((({47AE8D12-4C63-8F78-A873-14B28088BC95}-{9E98F76C-40DF-D2C0-F41C-FFA1BDB50911})*4.000000)+{FAA1E102-41F5-6835-B521-2392B542D801}))))
    (:then_8
      ;[1 1 1] Step 9
      (Variables|Default|SetSolTime (|({AFFBD59E-4A83-2DA1-CC5D-2181EB050192}+({AF0BBD6C-4979-7E9B-0730-D397F7DBCD6A}/60.000000)))))
    (:then_9
      ;[1 1 1] Step 10
      (Variables|Default|SetHra (|(({B7EADD58-40B4-BDB8-32CF-E6B7CA0BF54A}-12.000000)*15.000000))))
    (:then_10
      ;[1 1 1] Step 11
      (Variables|Default|SetDecl (|(23.452293*(SINd(((360.000000/365.242004)*({DE2DE248-49E9-199D-EFBD-C0972F14DAD7}-81.000000))))))))
    (:then_11
      ;[1 1 1] Step 12
      (Variables|Default|SetSAA (|(ASINd((((SINd({6C94AEFD-4628-E880-E38C-53B212950C21}))*(SINd({99211AF0-42B7-8C26-31A2-64A949AB99E5})))+(((COSd({6C94AEFD-4628-E880-E38C-53B212950C21}))*(COSd({99211AF0-42B7-8C26-31A2-64A949AB99E5})))*(COSd({A5A3EA6C-418B-3A90-6717-829A1DC6400C})))))))))
    (:then_12
      ;[1 1 1] Step 13
      (Variables|Default|SetSaz (|(ACOSd(((((SINd({6C94AEFD-4628-E880-E38C-53B212950C21}))*(COSd({99211AF0-42B7-8C26-31A2-64A949AB99E5})))-(((COSd({6C94AEFD-4628-E880-E38C-53B212950C21}))*(SINd({99211AF0-42B7-8C26-31A2-64A949AB99E5})))*(COSd({A5A3EA6C-418B-3A90-6717-829A1DC6400C}))))/(COSd({A99DC7A9-462C-0747-626E-3D9AAFC98D94})))))))
      (if (>= (Variables|Default|GetHra) 0.0)
        (Variables|Default|SetSaz (* (Variables|Default|GetSaz) -1.0))))
    (:then_13
      ;[1 1 1] Last Step
      (bind _output_get (Variables|Default|SetResult (Math|Rotator|MakeRotator 0.0 (- (Variables|Default|GetSAA) 1.8e+02) (Variables|Default|GetSaz))))
      (return _output_get))))

(fn CalculateTrajectoryCircular
  (params (Hour :type Integer) (Minute :type Integer) (Second :type Integer))
  (bind _longtime (CallFunction|GetLongTime Hour Minute Second))
  (bind _returnvalue (Math|Float|MapRangeClamped _longtime 12.0 23.99 -9e+01 9e+01))
  (bind _returnvalue_2 (Math|Float|MapRangeClamped _longtime 0.0 11.99 9e+01 -9e+01))
  (if (>= _longtime 12.0)
    (return (Math|Rotator|MakeRotator 0.0 _returnvalue (+ _returnvalue (Math|Float|MapRangeClamped _longtime 12.0 23.99 1e+02 6e+01))))
    (else
      (return (Math|Rotator|MakeRotator 0.0 _returnvalue_2 (- _returnvalue_2 (Math|Float|MapRangeClamped _longtime 0.0 11.99 6e+01 1e+02)))))))

(fn GetLongTime
  (params (Hour :type Integer) (Minute :type Integer) (Second :type Integer))
  (return (+ (Math|Conversions|ToFloat(Integer) Hour) (/ (Math|Conversions|ToFloat(Integer) Minute) 6e+01) (/ (Math|Conversions|ToFloat(Integer) Second) 3.6e+03))))