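; Cloudscape viewer actor that displays raymarched clouds on a mesh box, offset from landscape height or shrunk to a preview in development mode.
; MainConstruction pulls material instances and render targets from CloudscapeBuilderComponent, composites three layers into a coverage target, then feeds it with base, detail and turbulence textures to the raymarch material.
; It runs on construction and UpdateCloudscape; BeginPlay delays for render-target readiness before asking the builder to update.
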(event Custom|DoDelay
  (Utilities|FlowControl|Delay 0.0))

(event Custom|UpdateCloudscape
  (CallFunction|MainConstruction))

(event EventTick
  (params (DeltaSeconds :type Float%20%28single-precision%29)))

(event EventBeginPlay
  (bind _cloudscapebuildercomponent (Variables|Default|GetCloudscapeBuilderComponent))
  ;[1 1 1] Delay is necessary here too or you will have issues trying to use not ready rendertargets. Same comment at BP_CloudscapeSeasons.
  (CallFunction|DoDelay)
  (Utilities|FlowControl|ForLoopwithBreak 1 500 :!label _label
    (:LoopBody
      (bind _iscontructed (Class|BPICloudscapeBuilder|IsContructed(Message) _cloudscapebuildercomponent))
      (if (not (not _iscontructed))
        (goto _label Break)))
    (:Completed
      (Class|BPICloudscapeBuilder|UpdateCloudscape(Message) _cloudscapebuildercomponent))))

(fn ConstructionScript
  (bind _cloudscapebuildercomponent (Variables|Default|GetCloudscapeBuilderComponent))
  (Utilities|IsValid _cloudscapebuildercomponent
    (:Is%20Valid
      (bind _iscontructed (Class|BPICloudscapeBuilder|IsContructed(Message) _cloudscapebuildercomponent))
      (while (not _iscontructed)
        _)
      (if (Variables|Default|GetUpdate)
        (Variables|Default|SetUpdatePressed true))
      (Variables|Default|SetUpdate false)
      (CallFunction|MainConstruction))))

(fn MainConstruction
  (bind _mesh_scale_minimized (Variables|Default|GetMesh%20Scale%20Minimized))
  (bind _cloudscapemesh (Variables|Default|GetCloudscapeMesh))
  (bind _mesh_scale_maximized (Variables|Default|GetMesh%20Scale%20Maximized))
  (bind _cloudscapebuildercomponent (Variables|Default|GetCloudscapeBuilderComponent))
  (bind _landscape (Variables|Default|GetLandscape))
  (bind _cloudscapemesh_2 (Variables|Default|GetCloudscapeMesh))
  (bind _returnvalue (Transformation|GetWorldLocation _cloudscapemesh))
  (bind _returnvalue_2 (Transformation|GetWorldTransform _cloudscapemesh))
  (bind _max (Components|StaticMesh|GetLocalBounds _cloudscapemesh_2))
  (bind (_x _y) (Math|Vector|BreakVector _returnvalue))
  (bind _rotation (Math|Transform|BreakTransform _returnvalue_2))
  (bind _z (Math|Vector|BreakVector _max))
  (bind _returnvalue_3 (* _z _mesh_scale_maximized))
  (Utilities|IsValid _cloudscapebuildercomponent
    (:Is%20Valid
      (bind _iscontructed (Class|BPICloudscapeBuilder|IsContructed(Message) _cloudscapebuildercomponent))
      (while (not _iscontructed)
        _)
      (Utilities|IsValid _landscape
        (:Is%20Valid
          (Variables|Default|SetLandscapeHeight (.Z (Math|Vector|BreakVector (Transformation|GetActorLocation _landscape)))))
        (:Is%20Not%20Valid
          (Variables|Default|SetLandscapeHeight 0.0)))
      (Utilities|FlowControl|Sequence
        (:then_0
          (Variables|Default|SetOriginalPosition (Transformation|GetWorldLocation (Variables|Default|GetCloudscapeMesh))))
        (:then_1
          ;[1 1 1] Cloudscape Box Placement
          (if (and (Variables|Default|GetMinimizeCloudscape) (Variables|Default|GetDevelopmentMode))
            ;;[1 1 1] When minimized
            (Transformation|SetWorldTransform _cloudscapemesh (Math|Transform|MakeTransform "-900.000000,900.000000,450.000000" _rotation (Math|Vector|MakeVector _mesh_scale_minimized _mesh_scale_minimized _mesh_scale_minimized)) false true)
            (else
              (bind _verticalpositionadjustment (Class|BPICloudscapeBuilder|GetMeshVerticalPositionAdjustment(Message) (Variables|Default|GetCloudscapeBuilderComponent)))
              ;;[1 1 1] When not Minimized
              (Transformation|SetWorldTransform _cloudscapemesh (Math|Transform|MakeTransform (Math|Vector|MakeVector _x _y (+ (Math|Float|Lerp (* _returnvalue_3 -1.0) _returnvalue_3 _verticalpositionadjustment) (Variables|Default|GetClouscape%20Z-Axis%20offset) (Variables|Default|GetLandscapeHeight))) _rotation (Math|Vector|MakeVector _mesh_scale_maximized _mesh_scale_maximized _mesh_scale_maximized)) false true))))
        (:then_2
          (Rendering|SetVisibility (Variables|Default|GetCloudscapeMesh) (Variables|Default|GetVisible) false))
        (:then_3
          (bind _materials (Class|BPICloudscapeBuilder|GetCloudscapeMaterials(Message) (Variables|Default|GetCloudscapeBuilderComponent)))
          (for _array_element _materials
            (switch Utilities|FlowControl|Switch|SwitchonEMaterialTypes (.Type (Utilities|Struct|BreakSMaterials _array_element))
              (:NewEnumerator0
                (Variables|Default|SetCloudscapeMatInst (.MaterialInstance (Utilities|Struct|BreakSMaterials _array_element))))
              (:NewEnumerator1
                (Variables|Default|SetCloudscapeCoverageMatInst (.MaterialInstance (Utilities|Struct|BreakSMaterials _array_element))))
              (:NewEnumerator2
                (Variables|Default|SetCloudscapeLayer1MatInst (.MaterialInstance (Utilities|Struct|BreakSMaterials _array_element))))
              (:NewEnumerator3
                (Variables|Default|SetCloudscapeLayer2MatInst (.MaterialInstance (Utilities|Struct|BreakSMaterials _array_element))))
              (:NewEnumerator5
                (Variables|Default|SetCloudscapeLayer3MatInst (.MaterialInstance (Utilities|Struct|BreakSMaterials _array_element))))
              (:NewEnumerator6
                (Variables|Default|SetCloudscapeBaseMatInst (.MaterialInstance (Utilities|Struct|BreakSMaterials _array_element))))
              (:NewEnumerator7
                (Variables|Default|SetCloudscapeDetailsMatInst (.MaterialInstance (Utilities|Struct|BreakSMaterials _array_element))))
              (:NewEnumerator8
                (Variables|Default|SetCloudscapeTurbulenceMatInst (.MaterialInstance (Utilities|Struct|BreakSMaterials _array_element)))))))
        (:then_4
          (bind _rts (Class|BPICloudscapeBuilder|GetCloudscapeRenderTargets(Message) (Variables|Default|GetCloudscapeBuilderComponent)))
          (for _array_element_2 _rts
            (switch Utilities|FlowControl|Switch|SwitchonEMaterialTypes (.MaterialType (Utilities|Struct|BreakSRenderTargets _array_element_2))
              (:NewEnumerator1
                (Variables|Default|SetRTCoverage (.RenderTarget (Utilities|Struct|BreakSRenderTargets _array_element_2))))
              (:NewEnumerator2
                (Variables|Default|SetRTLayer1 (.RenderTarget (Utilities|Struct|BreakSRenderTargets _array_element_2))))
              (:NewEnumerator3
                (Variables|Default|SetRTLayer2 (.RenderTarget (Utilities|Struct|BreakSRenderTargets _array_element_2))))
              (:NewEnumerator5
                (Variables|Default|SetRTLayer3 (.RenderTarget (Utilities|Struct|BreakSRenderTargets _array_element_2))))
              (:NewEnumerator6
                (Variables|Default|SetRTBase (.RenderTarget (Utilities|Struct|BreakSRenderTargets _array_element_2))))
              (:NewEnumerator7
                (Variables|Default|SetRTDetails (.RenderTarget (Utilities|Struct|BreakSRenderTargets _array_element_2))))
              (:NewEnumerator8
                (Variables|Default|SetRTTurbulence (.RenderTarget (Utilities|Struct|BreakSRenderTargets _array_element_2)))))))
        (:then_5
          (Utilities|FlowControl|Sequence
            (:then_0
              (Utilities|IsValid (Variables|Default|GetCloudscapeCoverageMatInst)
                (:Is%20Valid
                  (Rendering|Material|SetTextureParameterValue (Variables|Default|GetCloudscapeCoverageMatInst) "LowCloudsTexture" (Variables|Default|GetRTLayer1)))))
            (:then_1
              (Utilities|IsValid (Variables|Default|GetCloudscapeCoverageMatInst)
                (:Is%20Valid
                  (Rendering|Material|SetTextureParameterValue (Variables|Default|GetCloudscapeCoverageMatInst) "MidCloudsTexture" (Variables|Default|GetRTLayer2)))))
            (:then_2
              (Utilities|IsValid (Variables|Default|GetCloudscapeCoverageMatInst)
                (:Is%20Valid
                  (Rendering|Material|SetTextureParameterValue (Variables|Default|GetCloudscapeCoverageMatInst) "HighCloudsTexture" (Variables|Default|GetRTLayer3)))))
            (:then_3
              (Rendering|ClearRenderTarget2D (Variables|Default|GetRTCoverage))
              (Rendering|DrawMaterialtoRenderTarget (Variables|Default|GetRTCoverage) (Variables|Default|GetCloudscapeCoverageMatInst))
              (Utilities|IsValid (Variables|Default|GetCloudscapeMatInst)
                (:Is%20Valid
                  (Rendering|Material|SetTextureParameterValue (Variables|Default|GetCloudscapeMatInst) "CloudCoverage" (Variables|Default|GetRTCoverage)))))
            (:then_4
              (Utilities|IsValid (Variables|Default|GetCloudscapeMatInst)
                (:Is%20Valid
                  (Rendering|Material|SetTextureParameterValue (Variables|Default|GetCloudscapeMatInst) "3DTexture_01" (Variables|Default|GetRTBase))
                  (Rendering|Material|SetTextureParameterValue (Variables|Default|GetCloudscapeMatInst) "3DTexture_02" (Variables|Default|GetRTDetails))
                  (Rendering|Material|SetTextureParameterValue (Variables|Default|GetCloudscapeMatInst) "2DTexture_01" (Variables|Default|GetRTTurbulence)))))
            (:then_5
              (Utilities|IsValid (Variables|Default|GetCloudscapeMatInst)
                (:Is%20Valid
                  (Rendering|Material|SetMaterial (Variables|Default|GetCloudscapeMesh) 0 (Variables|Default|GetCloudscapeMatInst)))))))
        (:then_6
          (Variables|Default|SetConstructed true))
        (:then_7
          (if (Variables|Default|GetUpdatePressed)
            (Variables|Default|SetUpdatePressed false)
            (Class|BPICloudscapeBuilder|UpdateCloudscape(Message) (Variables|Default|GetCloudscapeBuilderComponent))))))))

(fn SetVisible
  (params (IsVisible :type Boolean))
  (Variables|Default|SetVisible IsVisible))